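; Behavior tree task for AI vehicles that fires at the controller's current target, then hands execution to its parent task.
; When CurrentTarget is valid, each of the vehicle's weapon instances starts shooting if its aim target matches, otherwise it stops.
; Without a valid target, weapons are left untouched and only the parent logic runs.
; A failed cast to BP_AIVehicleController skips both the shooting and the parent call.
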(event EventReceiveExecuteAI
  (params (OwnerController :type AI%20Controller%20Object%20Reference) (ControlledPawn :type Pawn%20Object%20Reference))
  (bind _asbp_aivehicle_controller (Utilities|Casting|CastToBP_AIVehicleController OwnerController))
  (Utilities|IsValid (Variables|/Game/Blueprints/AI/BP_AIVehicleController.BP_AIVehicleController_C|GetCurrentTarget _asbp_aivehicle_controller)
    (:Is%20Valid
      (CallFunction|ShootTargetifCan (Variables|/Game/Blueprints/AI/BP_AIVehicleController.BP_AIVehicleController_C|GetControlledPawn _asbp_aivehicle_controller) (Variables|/Game/Blueprints/AI/BP_AIVehicleController.BP_AIVehicleController_C|GetCurrentTarget _asbp_aivehicle_controller)))
    (:Is%20Not%20Valid
      _))
  (|CallParentFunction OwnerController ControlledPawn))

(fn ShootTargetifCan
  (params (Shooter :type BP%20AI%20Vehicle%20Pawn%20Object%20Reference) (Shooting%20Target :type BP%20Vehicle%20Pawn%20Object%20Reference))
  (for _array_element (Default|GetWeaponInstances Shooter)
    (if (== (Class|WeaponInstance|GetAimTarget _array_element) Shooting%20Target)
      (Class|WeaponInstance|TryStartShooting _array_element)
      (else
        (Class|WeaponInstance|TryStopShooting _array_element)))))