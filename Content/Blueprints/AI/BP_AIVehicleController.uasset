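; AI controller for vehicle pawns that runs behavior tree logic and aims the vehicle's guns at its current target every tick.
; Perception updates pick a living, other-team vehicle in sight within a fixed range, keeping the last match rather than the nearest, and write it to the blackboard.
; MoveToLazy forwards move orders only when the destination shifts noticeably, and shares a valid, living pawn guard with targeting.
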(event OnPerceptionUpdated(AIPerceptionComponent)
  (params (UpdatedActors :type Array%20of%20Actor%20Object%20References))
  (CallFunction|UpdateTarget))

(event EventTick
  (params (DeltaSeconds :type Float%20%28single-precision%29))
  (bind _currenttarget (Variables|Default|GetCurrentTarget))
  (Utilities|IsValid _currenttarget
    (:Is%20Valid
      (Default|AimGuns (Variables|Default|GetControlledPawn) (Default|GetVehicleCenter _currenttarget)))))

(event EventPossess
  (params (PossessedPawn :type Pawn%20Object%20Reference))
  (bind _asbp_aivehicle_pawn (Utilities|Casting|CastToBP_AIVehiclePawn PossessedPawn)
    (:then
      (Variables|Default|SetControlledPawn _asbp_aivehicle_pawn)
      (AI|Logic|StartLogic (Variables|Default|GetBehaviorTreeComponent)))
    (:CastFailed
      (Development|PrintString "ERROR: Vehicle Controller can't be used on non-vehicle pawn"))))

(fn ConstructionScript)

(fn MovetoLazy
  (params (Location :type Vector))
  (Utilities|EnsureValidOwner
    (:out
      (if (> (Class|KismetMathLibrary|VectorDistanceSquared Location (Variables|/Game/Blueprints/AI/BP_AIVehiclePawn.BP_AIVehiclePawn_C|GetFinalTargetLocation (Variables|Default|GetControlledPawn))) 1e+05)
        (Default|Moveto (Variables|Default|GetControlledPawn) Location)))))

(fn UpdateTarget
  (Utilities|EnsureValidOwner
    (:out
      (Variables|Default|SetSquaredDistanceToTarget (Math|Float|Square 4e+04))
      (Variables|Default|SetCurrentTarget 0)
      (for _array_element (Class|AIPerceptionComponent|GetCurrentlyPerceivedActors (Variables|Default|GetAIPerceptionComponent) "/Script/AIModule.AISense_Sight")
        (bind _asbp_vehicle_pawn (Utilities|Casting|CastToBP_VehiclePawn _array_element))
        (if (not (or (== (Variables|/Game/Blueprints/Vehicle/BP_VehiclePawn.BP_VehiclePawn_C|GetTeam (Variables|Default|GetControlledPawn)) (Variables|/Game/Blueprints/Vehicle/BP_VehiclePawn.BP_VehiclePawn_C|GetTeam _asbp_vehicle_pawn)) (Variables|/Game/Blueprints/Vehicle/BP_VehiclePawn.BP_VehiclePawn_C|GetbDead _asbp_vehicle_pawn)))
          (if (< (Transformation|GetSquaredDistanceTo _asbp_vehicle_pawn) (Variables|Default|GetSquaredDistanceToTarget))
            (Variables|Default|SetCurrentTarget _asbp_vehicle_pawn))))
      (AI|Components|Blackboard|SetValueasObject (Variables|Default|GetBlackboardComponent) (Utilities|Name|MakeLiteralName "EnemyActor") (Variables|Default|GetCurrentTarget))
      (Utilities|DebugOnly
        (:DebugOnly
          (Development|PrintString (Utilities|String|Append "New target selected: " (Utilities|GetDisplayName (Variables|Default|GetCurrentTarget)))))))))