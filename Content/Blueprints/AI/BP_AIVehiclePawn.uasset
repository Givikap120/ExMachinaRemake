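; AI-driven vehicle pawn that follows its own spawned spline path, with halved preset HP and controller shutdown on death.
; MoveTo builds a ground-traced spline to the target.
; Tick steers toward a speed-scaled look-ahead point on it and sets throttle from yaw error.
; A forward box trace detects non-landscape obstacles, runs A* over a traced grid around each, and splices the detour into the spline.
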(event Custom|SetThrottle
  (params (Throttle :type Float%20%28double-precision%29))
  ;[1 1 1] Events
  (Utilities|EnsureAlive
    (:out
      (CallFunction|SetThrottleInternal Throttle))
    (:dead
      (CallFunction|SetThrottleInternal 0.0))))

(event Custom|SetBrake
  (params (Brake :type Float%20%28double-precision%29))
  ;[1 1 1] Events
  (Utilities|EnsureAlive
    (:out
      (Class|ChaosVehicleMovementComponent|SetBrakeInput (Variables|Default|GetVehicleMovementComponent) Brake))))

(event Custom|SetSteering
  (params (Steering :type Float%20%28double-precision%29))
  ;[1 1 1] Events
  (Utilities|EnsureAlive
    (:out
      (Class|ChaosVehicleMovementComponent|SetSteeringInput (Variables|Default|GetVehicleMovementComponent) Steering))))

(event Custom|SetHandbrake
  (params (HandBrake :type Boolean))
  ;[1 1 1] Events
  (Utilities|EnsureAlive
    (:out
      (Class|ChaosVehicleMovementComponent|SetHandbrakeInput (Variables|Default|GetVehicleMovementComponent) HandBrake))))

(event EventBeginPlay
  (bind _self self)
  (|CallParentFunction)
  (Variables|Default|SetAttackRangeSquareed (Math|Float|Square (Math|Float|Max(Float) (Class|VehiclePart|GetFiringRange (Variables|Default|GetCabin)) (Class|VehiclePart|GetFiringRange (Variables|Default|GetCargo)))))
  (bind _returnvalue (Game|SpawnActorfromClass "/Game/Blueprints/AI/BP_SplinePath.BP_SplinePath_C" (Transformation|GetActorTransform) "AlwaysSpawn" "MultiplyWithRoot" _self _self))
  (Variables|Default|SetSpline _returnvalue))

(event Collision|EventActorBeginOverlap
  (params (OtherActor :type Actor%20Object%20Reference)))

(event EventTick
  (params (DeltaSeconds :type Float%20%28single-precision%29))
  (bind _vehiclehalfsize (Variables|Default|GetVehicleHalfSize))
  (Utilities|EnsureAlive
    (:out
      (|CallParentFunction DeltaSeconds)
      (bind _steering (Private|CalculateSteeringInput))
      (CallFunction|SetSteering _steering)
      (Private|UpdateObstaclePath)
      (if (>= (Math|Float|MapRangeClamped (Math|Float|Absolute(Float) (Variables|Steering|GetYawDelta)) 3e+01 5.0 (Variables|Steering|GetMinSpeed) (Variables|Steering|GetMaxSpeed)) (Vehicle|GetForwardSpeed (Variables|Default|GetVehicleMovementComponent)))
        (CallFunction|SetThrottle 1.0)
        (else
          (CallFunction|SetThrottle -1.0)))
      (Obstacle|HandleFrontObstacle (.y _vehiclehalfsize) (.z _vehiclehalfsize)))))

(event EventHandleDeath
  (|CallParentFunction)
  (bind _asbp_aivehicle_controller (Utilities|Casting|CastToBP_AIVehicleController (Pawn|GetController)))
  (AI|Logic|StopLogic (Variables|/Game/Blueprints/AI/BP_AIVehicleController.BP_AIVehicleController_C|GetBehaviorTreeComponent _asbp_aivehicle_controller) "Owner is dead")
  (Pawn|UnPossess _asbp_aivehicle_controller)
  (Actor|Tick|SetActorTickEnabled _asbp_aivehicle_controller))

(fn ConstructionScript
  (|CallParentFunction))

(fn GetNearestSpline
  (params (Splines :type Array%20of%20BP%20Spline%20Path%20Object%20References))
  (bind _returnvalue (Transformation|GetActorLocation))
  (LocalVariables|SetDistance 0.0)
  (for (_array_element _array_index) Splines
    (if (== _array_index 0)
      (LocalVariables|SetDistance (Math|Vector|Distance(Vector) (Spline|FindLocationClosesttoWorldLocation (Variables|/Game/Blueprints/AI/BP_SplinePath.BP_SplinePath_C|GetSpline _array_element) _returnvalue "World") _returnvalue) :!label _label)
      (LocalVariables|SetNearestSpline _array_element)
      (elif (< (Math|Vector|Distance(Vector) (Spline|FindLocationClosesttoWorldLocation (Variables|/Game/Blueprints/AI/BP_SplinePath.BP_SplinePath_C|GetSpline _array_element) _returnvalue "World") _returnvalue) (LocalVariables|GetDistance))
        (goto _label))))
  (return (LocalVariables|GetNearestSpline)))

(fn CalculateSteeringInput
  (bind _returnvalue (Transformation|GetActorLocation))
  (bind _returnvalue_2 (Transformation|GetActorLocation))
  (bind _output_get (Variables|Steering|SetOffsetTangentLocation (Spline|FindLocationClosesttoWorldLocation (Variables|/Game/Blueprints/AI/BP_SplinePath.BP_SplinePath_C|GetSpline (Variables|Default|GetSpline)) (+ _returnvalue (* (Math|Vector|Normalize (Class|SplineComponent|FindTangentClosesttoWorldLocation (Variables|/Game/Blueprints/AI/BP_SplinePath.BP_SplinePath_C|GetSpline (Variables|Default|GetSpline)) _returnvalue "World")) (+ (Vehicle|GetForwardSpeed (Variables|Default|GetVehicleMovementComponent)) (* (.y (Variables|Default|GetVehicleHalfSize)) 4.0)))) "World")))
  (Utilities|DebugSwitch
    (:Debug
      (Rendering|Debug|DrawDebugSphere _output_get 1e+02 12 "(R=1.000000,G=0.000000,B=0.000000,A=1.000000)" 0.0 1.0)
      (Rendering|Debug|DrawDebugArrow :LineStart _returnvalue_2 :LineEnd _output_get))
    (:Normal
      _))
  (bind _output_get_2 (Variables|Steering|SetYawDelta (.yaw (Math|Rotator|Delta(Rotator) (Math|Rotator|FindLookatRotation _returnvalue_2 _output_get) (Transformation|GetActorRotation)))))
  (return (Math|Float|MapRangeClamped _output_get_2 -15.0 15.0 -1.0 1.0)))

(fn Moveto
  (params (Position :type Vector))
  (Utilities|DebugSwitch
    (:Debug
      (Rendering|Debug|DrawDebugSphere Position 1e+02 12 "(R=1.000000,G=1.000000,B=1.000000,A=1.000000)" 1.0))
    (:Normal
      _))
  (Variables|Default|SetFinalTargetLocation Position)
  (Private|CreateMovetoSpline)
  (Spline|SetSplinePoints (Variables|/Game/Blueprints/AI/BP_SplinePath.BP_SplinePath_C|GetSpline (Variables|Default|GetSpline)) (Variables|Default|GetMoveToPath) "World" true)
  (Obstacle|InjectPathinSpline (Variables|Default|GetLastObstaclePath)))

(fn CreateMovetoSpline
  (bind _returnvalue (Transformation|GetActorLocation))
  (bind _movetopath (Variables|Default|GetMoveToPath))
  (bind _finaltargetlocation (Variables|Default|GetFinalTargetLocation))
  (bind _vehiclehalfsize (Variables|Default|GetVehicleHalfSize))
  (bind _gridgap (Variables|Default|GetGridGap))
  (bind _z (Math|Vector|BreakVector _returnvalue))
  (LocalVariables|SetCurrentLocation _returnvalue)
  (LocalVariables|SetMinTraceZ (- (Math|Float|Min(Float) (.z _finaltargetlocation) _z) (.z _vehiclehalfsize)))
  (LocalVariables|SetMaxTraceZ (+ (Math|Float|Max(Float) (.z _finaltargetlocation) _z) (.z _vehiclehalfsize)))
  (Utilities|Array|Clear _movetopath)
  (Utilities|Array|Add _movetopath _returnvalue)
  (LocalVariables|SetStep (Math|Conversions|ToVector2D(Vector) (* (Math|Vector|GetUnitDirection(Vector) (LocalVariables|GetCurrentLocation) (Variables|Default|GetFinalTargetLocation)) _gridgap)))
  (while (> (Math|Vector|Distance2D(Vector) (Math|Conversions|ToVector2D(Vector) (LocalVariables|GetCurrentLocation)) (Math|Conversions|ToVector2D(Vector) (Variables|Default|GetFinalTargetLocation))) _gridgap)
    (LocalVariables|SetCurrentLocation (+ (LocalVariables|GetCurrentLocation) (LocalVariables|GetStep)))
    (bind (_outhit _returnvalue_2) (Collision|LineTraceByChannel (Math|Vector|MakeVector (.x (LocalVariables|GetCurrentLocation)) (.y (LocalVariables|GetCurrentLocation)) (LocalVariables|GetMinTraceZ)) (Math|Vector|MakeVector (.x (LocalVariables|GetCurrentLocation)) (.y (LocalVariables|GetCurrentLocation)) (LocalVariables|GetMaxTraceZ)) "TraceTypeQuery1" false 0 "None"))
    (if _returnvalue_2
      (LocalVariables|SetCurrentLocation (Math|Vector|MakeVector (.x (LocalVariables|GetCurrentLocation)) (.y (LocalVariables|GetCurrentLocation)) (.z (.location _outhit)))))
    (Utilities|Array|Add (Variables|Default|GetMoveToPath) (LocalVariables|GetCurrentLocation)))
  (if (> (Math|Vector|Distance(Vector) (LocalVariables|GetCurrentLocation) (Variables|Default|GetFinalTargetLocation)) (* (Variables|Default|GetGridGap) 0.2))
    (Utilities|Array|Add (Variables|Default|GetMoveToPath) (Variables|Default|GetFinalTargetLocation))))

(fn HandleFrontObstacle
  (params (Front%20Offset :type Float%20%28double-precision%29) (Height%20Offset :type Float%20%28double-precision%29))
  (bind _returnvalue (Transformation|GetActorLocation))
  (bind _returnvalue_2 (Transformation|GetActorForwardVector))
  (bind _returnvalue_3 (* _returnvalue_2 Front%20Offset))
  (bind _returnvalue_4 (+ _returnvalue _returnvalue_3))
  (bind _returnvalue_5 (+ (.z _returnvalue_4) Height%20Offset))
  (bind _returnvalue_6 (Math|Vector|MakeVector (.x _returnvalue_4) (.y _returnvalue_4) _returnvalue_5))
  (bind _result (Utilities|GetDebugDrawType "ForOneFrame")
    (:Out
      (bind (_outhit _returnvalue_7) (Collision|BoxTraceByChannel _returnvalue_6 (+ _returnvalue_6 (Class|KismetMathLibrary|CreateVectorfromYawPitch (.yaw (Pawn|GetControlRotation :!class /Script/Engine.Pawn)) 0.0 (+ (Vehicle|GetForwardSpeed (Variables|Default|GetVehicleMovementComponent)) 1e+03))) (Variables|Default|GetVehicleHalfSize) (Transformation|GetActorRotation) "TraceTypeQuery1" false (Variables|Default|GetProcessed%20Objects) _result))
      (if _returnvalue_7
        (Class|KismetSystemLibrary|IsObjectOfSoftClass (.HitActor (Collision|BreakHitResult _outhit)) "/Script/Landscape.Landscape"
          (:False
            (bind _points (Obstacle|BuildGridPoints (.HitActor (Collision|BreakHitResult _outhit))))
            (bind _path (Obstacle|PathFind _points))
            (Variables|Default|SetLastObstaclePath _path)
            (Obstacle|InjectPathinSpline _path)
            (Utilities|Array|Add (Variables|Default|GetProcessed%20Objects) (.HitActor (Collision|BreakHitResult _outhit)))))))))

(fn BuildGridPoints
  (params (Obstacle :type Actor%20Object%20Reference))
  (bind _gridcount (Variables|Default|GetGridCount))
  (bind _gridgap (Variables|Default|GetGridGap))
  (bind _gridpoints (LocalVariables|GetGridPoints))
  (bind _returnvalue (* _gridcount -1))
  (bind _output_get (LocalVariables|SetGridCenter (Transformation|GetActorLocation Obstacle)))
  (for _index (range _returnvalue _gridcount)
    (Utilities|Array|Clear (LocalVariables|GetRowPoints))
    (for _index_2 (range _returnvalue _gridcount)
      (bind _point (Private|GetGridPoint (+ _output_get (Math|Vector|MakeVector (* _index _gridgap) (* _index_2 _gridgap) 0.0))))
      (Utilities|Array|Add (LocalVariables|GetRowPoints) _point))
    (Utilities|Array|Add _gridpoints (Utilities|Struct|MakePointRow (LocalVariables|GetRowPoints))))
  (return _gridpoints))

(fn GetGridPoint
  (params (Source :type Vector))
  (bind (_outhit _returnvalue) (Collision|LineTraceForObjects (Math|Vector|MakeVector (.x Source) (.y Source) (+ (.z Source) 1e+04)) (Math|Vector|MakeVector (.x Source) (.y Source) (- (.z Source) 1e+04)) (Utilities|Array|MakeArray (Utilities|Enum|LiteralenumEObjectTypeQuery "ObjectTypeQuery1")) false 0 "None"))
  (if _returnvalue
    (Utilities|DebugSwitch
      (:Debug
        (Rendering|Debug|DrawDebugSphere (.Location (Collision|BreakHitResult _outhit)) 1e+02 12 "(R=1.000000,G=0.000000,B=0.000000,A=1.000000)" 1e+01 5.0))
      (:Normal
        _))
    (return (.Location (Collision|BreakHitResult _outhit)))
    (else
      (return Source))))

(fn UpdateObstaclePath
  (bind _spline (Variables|Default|GetSpline))
  (bind _spline_2 (Variables|/Game/Blueprints/AI/BP_SplinePath.BP_SplinePath_C|GetSpline _spline))
  (if (Utilities|Array|IsNotEmpty (Variables|Default|GetLastObstaclePath))
    (LocalVariables|SetMinDistance (Math|Float|Square 9999999.0))
    (for _index (range 0 (- (Spline|GetNumberOfSplinePoints _spline_2) 1))
      (if (< (Class|KismetMathLibrary|VectorDistanceSquared (Spline|GetLocationatSplinePoint _spline_2 _index "World") (Transformation|GetActorLocation)) (LocalVariables|GetMinDistance))
        (LocalVariables|SetMinDistance (Class|KismetMathLibrary|VectorDistanceSquared (Spline|GetLocationatSplinePoint _spline_2 _index "World") (Transformation|GetActorLocation)))
        (LocalVariables|SetMinPoint (Spline|GetLocationatSplinePoint _spline_2 _index "World"))))
    (bind _returnvalue (Utilities|Array|RemoveItem (Variables|Default|GetLastObstaclePath) (LocalVariables|GetMinPoint)))
    (if _returnvalue
      (Utilities|DebugOnly
        (:DebugOnly
          (Development|PrintString "Point Removed"))))))

(fn Reload
  (for _array_element (CallFunction|GetActiveWeapons)
    _))

(fn GetActiveWeapons
  (bind _cabin (Variables|Default|GetCabin))
  (bind _cargo (Variables|Default|GetCargo))
  (bind _result_weapons (LocalVariables|GetResult%20Weapons))
  (bind _returnvalue (Class|VehiclePart|GetWeapon _cargo))
  (bind _returnvalue_2 (Class|VehiclePart|GetWeapon _cabin))
  (Utilities|IsValid _returnvalue_2
    (:Is%20Valid
      (Utilities|Array|Add _result_weapons _returnvalue_2))
    (:Is%20Not%20Valid
      _))
  (Utilities|IsValid _returnvalue
    (:Is%20Valid
      (Utilities|Array|Add _result_weapons _returnvalue))
    (:Is%20Not%20Valid
      _))
  (return 0))

(fn PathFind
  (params (Points :type Array%20of%20Point%20Row%20Structures))
  (bind _output_get (LocalVariables|SetClosestToStartDistance (Math|Float|Square 9999999.0)))
  (LocalVariables|SetClosestToEndDistance _output_get)
  (for _array_element Points
    (for _array_element_2 (Utilities|Struct|BreakPointRow _array_element)
      (if (< (Class|KismetMathLibrary|VectorDistanceSquared _array_element_2 (Transformation|GetActorLocation)) (LocalVariables|GetClosestToStartDistance))
        (LocalVariables|SetClosestToStart _array_element_2)
        (LocalVariables|SetClosestToStartDistance (Class|KismetMathLibrary|VectorDistanceSquared _array_element_2 (Transformation|GetActorLocation)))
        (elif (< (Class|KismetMathLibrary|VectorDistanceSquared _array_element_2 (Variables|Default|GetFinalTargetLocation)) (LocalVariables|GetClosestToEndDistance))
          (LocalVariables|SetClosestToEnd _array_element_2)
          (LocalVariables|SetClosestToEndDistance (Class|KismetMathLibrary|VectorDistanceSquared _array_element_2 (Variables|Default|GetFinalTargetLocation)))))))
  (bind (_outpath _returnvalue) (Class|CustomFunctionLibrary|AStarPathfinding Points (LocalVariables|GetClosestToStart) (LocalVariables|GetClosestToEnd) (Variables|Default|GetVehicleHalfSize) 45.0))
  (if _returnvalue
    (Utilities|DebugSwitch
      (:Debug
        (Obstacle|DebugDrawPath _outpath))
      (:Normal
        _))
    (return _outpath)))

(fn InjectPathinSpline
  (params (Path :type Array%20of%20Vectors))
  (bind _spline (Variables|Default|GetSpline))
  (bind _spline_2 (Variables|Default|GetSpline))
  (bind _spline_3 (Variables|/Game/Blueprints/AI/BP_SplinePath.BP_SplinePath_C|GetSpline _spline))
  (bind _spline_4 (Variables|/Game/Blueprints/AI/BP_SplinePath.BP_SplinePath_C|GetSpline _spline_2))
  (if (Utilities|Array|IsNotEmpty Path)
    (bind _output_get (LocalVariables|SetClosestStartPointDistance (Math|Float|Square 9999999.0)))
    (LocalVariables|SetClosestEndPointDistance _output_get)
    (LocalVariables|SetPathStart (Utilities|Array|Get(acopy) Path))
    (LocalVariables|SetPathEnd (Utilities|Array|Get(acopy) Path (Utilities|Array|LastIndex Path)))
    (for _index (range 0 (- (Spline|GetNumberOfSplinePoints _spline_3) 1))
      (if (< (Class|KismetMathLibrary|VectorDistanceSquared (Spline|GetLocationatSplinePoint _spline_3 _index "World") (LocalVariables|GetPathStart)) (LocalVariables|GetClosestStartPointDistance))
        (LocalVariables|SetClosestStartPoint _index)
        (LocalVariables|SetClosestStartPointDistance (Class|KismetMathLibrary|VectorDistanceSquared (Spline|GetLocationatSplinePoint _spline_3 _index "World") (LocalVariables|GetPathStart))))
      (if (< (Class|KismetMathLibrary|VectorDistanceSquared (Spline|GetLocationatSplinePoint _spline_3 _index "World") (LocalVariables|GetPathEnd)) (LocalVariables|GetClosestEndPointDistance))
        (LocalVariables|SetClosestEndPoint _index)
        (LocalVariables|SetClosestEndPointDistance (Class|KismetMathLibrary|VectorDistanceSquared (Spline|GetLocationatSplinePoint _spline_3 _index "World") (LocalVariables|GetPathEnd)))))
    (LocalVariables|SetClosestEndPoint (Math|Integer|Max(Integer) (LocalVariables|GetClosestStartPoint) (LocalVariables|GetClosestEndPoint)))
    (LocalVariables|Seti (- (LocalVariables|GetClosestEndPoint) 1))
    (while (> (LocalVariables|Geti) (LocalVariables|GetClosestStartPoint))
      (Spline|RemoveSplinePoint _spline_4 (LocalVariables|Geti) false)
      (Math|Integer|DecrementInt (LocalVariables|Geti)))
    (for (_array_element _array_index) Path
      (Spline|AddSplinePointatIndex _spline_4 _array_element (+ (LocalVariables|GetClosestStartPoint) _array_index 1) "World" false))
    (Spline|UpdateSpline _spline_4)))

(fn EnsureObstaclePathValid
  (bind _returnvalue (Transformation|GetActorLocation))
  (bind _lastobstaclepath (Variables|Default|GetLastObstaclePath))
  (if (not (Utilities|Array|IsEmpty _lastobstaclepath))
    (if (<= (Class|KismetMathLibrary|VectorDistanceSquared _returnvalue (Variables|Default|GetFinalTargetLocation)) (Class|KismetMathLibrary|VectorDistanceSquared _returnvalue (Utilities|Array|Get(acopy) _lastobstaclepath (Utilities|Array|LastIndex _lastobstaclepath))))
      (Utilities|Array|Clear (Variables|Default|GetLastObstaclePath)))))

(fn DebugDrawPath
  (params (Path :type Array%20of%20Vectors))
  (for (_array_element _array_index) Path
    (if (== _array_index 0)
      _
      (else
        (Rendering|Debug|DrawDebugLine (LocalVariables|GetPrev) _array_element "(R=0.000000,G=0.145196,B=1.000000,A=1.000000)" 1e+01 5.0)))
    (LocalVariables|SetPrev _array_element)))

(fn InitCarfromPreset
  (|CallParentFunction)
  (Variables|Default|SetCurrentHP (/ (Variables|Default|GetCurrentHP) 2)))