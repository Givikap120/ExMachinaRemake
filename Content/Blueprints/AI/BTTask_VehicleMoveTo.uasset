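; Behavior tree task that moves an AI vehicle toward its controller's current target and reports whether it is in attack range.
; A living target gets a lazy move to its location, and a squared-distance check sets the in-range blackboard key and the task result.
; A dead target makes the vehicle move to its own position, request a target update and fail.
; An invalid target leaves the task unfinished.
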(event EventReceiveExecuteAI
  (params (OwnerController :type AI%20Controller%20Object%20Reference) (ControlledPawn :type Pawn%20Object%20Reference))
  (bind _asbp_aivehicle_controller (Utilities|Casting|CastToBP_AIVehicleController OwnerController))
  (Utilities|IsValid (Variables|/Game/Blueprints/AI/BP_AIVehicleController.BP_AIVehicleController_C|GetCurrentTarget _asbp_aivehicle_controller)
    (:Is%20Valid
      (if (Variables|/Game/Blueprints/Vehicle/BP_VehiclePawn.BP_VehiclePawn_C|GetbDead (Variables|/Game/Blueprints/AI/BP_AIVehicleController.BP_AIVehicleController_C|GetCurrentTarget _asbp_aivehicle_controller))
        (Default|MovetoLazy _asbp_aivehicle_controller (Transformation|GetActorLocation (Variables|/Game/Blueprints/AI/BP_AIVehicleController.BP_AIVehicleController_C|GetControlledPawn _asbp_aivehicle_controller)))
        (Default|UpdateTarget _asbp_aivehicle_controller)
        (AI|BehaviorTree|FinishExecute false)
        (else
          (Default|MovetoLazy _asbp_aivehicle_controller (Transformation|GetActorLocation (Variables|/Game/Blueprints/AI/BP_AIVehicleController.BP_AIVehicleController_C|GetCurrentTarget _asbp_aivehicle_controller)))
          (Class|BTFunctionLibrary|SetBlackboardValueasBool (Variables|Default|GetTargetInRangeKey) (< (Transformation|GetSquaredDistanceTo (Variables|/Game/Blueprints/AI/BP_AIVehicleController.BP_AIVehicleController_C|GetCurrentTarget _asbp_aivehicle_controller) (Variables|/Game/Blueprints/AI/BP_AIVehicleController.BP_AIVehicleController_C|GetControlledPawn _asbp_aivehicle_controller)) (Variables|/Game/Blueprints/AI/BP_AIVehiclePawn.BP_AIVehiclePawn_C|GetAttackRangeSquareed (Variables|/Game/Blueprints/AI/BP_AIVehicleController.BP_AIVehicleController_C|GetControlledPawn _asbp_aivehicle_controller))))
          (AI|BehaviorTree|FinishExecute (< (Transformation|GetSquaredDistanceTo (Variables|/Game/Blueprints/AI/BP_AIVehicleController.BP_AIVehicleController_C|GetCurrentTarget _asbp_aivehicle_controller) (Variables|/Game/Blueprints/AI/BP_AIVehicleController.BP_AIVehicleController_C|GetControlledPawn _asbp_aivehicle_controller)) (Variables|/Game/Blueprints/AI/BP_AIVehiclePawn.BP_AIVehiclePawn_C|GetAttackRangeSquareed (Variables|/Game/Blueprints/AI/BP_AIVehicleController.BP_AIVehicleController_C|GetControlledPawn _asbp_aivehicle_controller)))))))))