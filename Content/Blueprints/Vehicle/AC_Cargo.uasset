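; AC_Cargo is a vehicle part component that gives a vehicle cargo storage through an owned, grid-based Inventory object.
; Its stats load from the TCargo data table by row name, which also initializes the weapon slot and sets the inventory's X/Y capacity.
; It wraps inventory placement, removal and validation, and extends parent item queries, clearing and part save/load to include the cargo contents.
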(event EventBeginPlay
  (|CallParentFunction)
  (bind _returnvalue (Class|CustomFunctionLibrary|CreateObject "/Script/ExMachinaRemake.Inventory"))
  (Variables|Default|SetInventory (.AsInventory (Utilities|Casting|CastToInventory _returnvalue))))

(event EventTick
  (params (DeltaSeconds :type Float%20%28single-precision%29)))

(fn SetfromCargo
  (params (Name :type Name))
  (bind _returnvalue (Utilities|GetDataTableRow "/Game/Tables/TCargo.TCargo" Name)
    (:then
      (Variables|Default|SetPart%20Stats (.partstats _returnvalue))
      (Variables|Default|SetCargoStats (.cargostats _returnvalue))
      (CallFunction|InitWeaponSlot)
      (CallFunction|InitInventoryifNeeded))))

(fn RemoveItembyCoords
  (params (PosX :type Integer) (PosY :type Integer))
  (bind _returnvalue (Class|Inventory|RemoveItemat (Variables|Default|GetInventory) PosX PosY))
  (return (Utilities|IsValid _returnvalue)))

(fn TryAddItemtoInventory
  (params (Item :type Item%20Object%20Reference) (X_Index :type Integer) (Y_Index :type Integer))
  (bind _returnvalue (Class|Inventory|TryPlaceItem (Variables|Default|GetInventory) Item X_Index Y_Index))
  (return _returnvalue))

(fn TryDropItemtoInventory
  (params (Item :type Item%20Object%20Reference))
  (bind _inventory (Variables|Default|GetInventory))
  (Utilities|IsValid _inventory
    (:Is%20Valid
      (bind _returnvalue (Class|Inventory|TryDropItemInside _inventory Item))
      (return _returnvalue))))

(fn ValidateCargo
  (Class|Inventory|Validate (Variables|Default|GetInventory)))

(fn GetInventory
  (return (Variables|Default|GetInventory)))

(fn GetInventoryItems
  (return (Variables|/Script/ExMachinaRemake.Inventory|GetItems (Variables|Default|GetInventory))))

(fn InitInventoryifNeeded
  (bind _cargostats (Variables|Default|GetCargoStats))
  (bind (_capacityx _capacityy) (Utilities|Struct|BreakF_CargoBase_Stats _cargostats))
  (Utilities|IsValid (Variables|Default|GetInventory)
    (:Is%20Valid
      _)
    (:Is%20Not%20Valid
      (bind _returnvalue (Class|CustomFunctionLibrary|CreateObject "/Script/ExMachinaRemake.Inventory"))
      (bind _output_get (Variables|Default|SetInventory (.AsInventory (Utilities|Casting|CastToInventory _returnvalue))))))
  (Variables|/Script/ExMachinaRemake.Inventory|SetCapacityX _output_get _capacityx)
  (Variables|/Script/ExMachinaRemake.Inventory|SetCapacityY _output_get _capacityy))

(fn GetAllItems
  (bind _output_get (LocalVariables|SetResultItems (|CallParentFunction)))
  (for _array_element (Pure|GetInventoryItems)
    (Utilities|Array|Add _output_get (.item _array_element)))
  (return _output_get))

(fn InitComponents
  (|CallParentFunction)
  (CallFunction|InitInventoryifNeeded))

(fn SaveCargo
  (return (Utilities|Struct|MakeF_SaveGame_Cargo (CallFunction|SaveVehiclePart) (Variables|Default|GetCargoStats) (Class|Inventory|SaveInventory (Variables|Default|GetInventory)))))

(fn LoadCargo
  (params (Load :type F%20Save%20Game%20Cargo%20Structure))
  (Variables|Default|SetCargoStats (.cargostats Load))
  (CallFunction|LoadVehiclePart (.vehiclepartdata Load))
  (Class|Inventory|LoadInventory (Variables|Default|GetInventory) (.inventorydata Load)))

(fn RemoveAllItems
  (|CallParentFunction)
  (Class|Inventory|Clear (Variables|Default|GetInventory)))

(fn HasItem
  (params (Item :type Item%20Object%20Reference))
  (return (or (|CallParentFunction Item) (Class|Inventory|HasItem (Variables|Default|GetInventory) Item))))