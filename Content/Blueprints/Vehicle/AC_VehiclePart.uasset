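; Vehicle part component that holds part stats and a weapon slot, handling the part's mesh, pricing and weapon.
; InitComponents creates or refreshes the WeaponSlot from PartStats and applies the mesh.
; The slot holds the weapon item, while a separate weapon instance is initialized from it and aimed at targets.
; Save and load round-trip part and weapon stats, and a dummy weapon stands in for cost totals when the slot is empty.
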(event EventBeginPlay)

(event EventTick
  (params (DeltaSeconds :type Float%20%28single-precision%29)))

(fn TryRotateGuns
  (params (Target%20Location :type Vector))
  (bind _weaponinstanceref (Variables|Default|GetWeaponInstanceRef))
  (if (and (Class|WeaponSlot|HasWeapon (Variables|Default|GetWeaponSlot)) (Utilities|IsValid _weaponinstanceref))
    (Class|WeaponInstance|Aimto _weaponinstanceref Target%20Location)))

(fn UpdateWeapon
  (if (Utilities|IsValid (Variables|Default|GetWeaponInstanceRef))
    (Class|WeaponInstance|InitializefromWeapon (Variables|Default|GetWeaponInstanceRef) (Variables|/Script/ExMachinaRemake.WeaponSlot|GetWeapon (Variables|Default|GetWeaponSlot)))))

(fn RemoveAllItems
  (Class|WeaponSlot|RemoveWeapon (Variables|Default|GetWeaponSlot)))

(fn TryDropWeapontoSlot
  (params (Weapon :type BP%20Weapon%20Object%20Reference))
  (bind _returnvalue (Class|WeaponSlot|TryDropWeapon (Variables|Default|GetWeaponSlot) Weapon))
  (return _returnvalue))

(fn InitWeaponSlot
  (Utilities|IsValid (Variables|Default|GetWeaponSlot)
    (:Is%20Valid
      _)
    (:Is%20Not%20Valid
      (bind _returnvalue (Class|CustomFunctionLibrary|CreateObject "/Script/ExMachinaRemake.WeaponSlot"))
      (bind _output_get (Variables|Default|SetWeaponSlot (.AsWeapon%20Slot (Utilities|Casting|CastToWeaponSlot _returnvalue))))
      (EventDispatchers|BindEventtoOnWeaponChanged _output_get (EventDispatchers|CreateEvent :!event UpdateWeapon))))
  (Class|WeaponSlot|SetfromStats _output_get (Utilities|Struct|BreakF_VehiclePart_Stats (Variables|Default|GetPart%20Stats)))
  (return _output_get))

(fn InitComponents
  (bind _mesh_ref (Variables|Default|GetMesh%20Ref))
  (Technical|InitWeaponSlot)
  (Utilities|IsValid _mesh_ref
    (:Is%20Valid
      (CallFunction|SetStaticMeshandMaterials _mesh_ref (Utilities|Struct|BreakF_VehiclePart_Stats (Variables|Default|GetPart%20Stats))))))

(fn ValidateSlots
  (bind _returnvalue (Class|WeaponSlot|ValidateWeapon (Variables|Default|GetWeaponSlot)))
  (return (.AsBP%20Weapon (Utilities|Casting|CastToBP_Weapon _returnvalue))))

(fn GetWeapon
  (return (.AsBP%20Weapon (Utilities|Casting|CastToBP_Weapon (Variables|/Script/ExMachinaRemake.WeaponSlot|GetWeapon (Variables|Default|GetWeaponSlot))))))

(fn GetWeaponSafe
  (bind _weaponslot (Variables|Default|GetWeaponSlot))
  (bind _weapon (Variables|/Script/ExMachinaRemake.WeaponSlot|GetWeapon _weaponslot))
  (Utilities|IsValid _weapon
    (:Is%20Valid
      (return (.AsBP%20Weapon (Utilities|Casting|CastToBP_Weapon _weapon))))
    (:Is%20Not%20Valid
      (bind _returnvalue (Class|CustomFunctionLibrary|CreateObject "/Game/BP_C++/BP_DummyWeapon.BP_DummyWeapon_C"))
      (bind _asbp_weapon (Utilities|Casting|CastToBP_Weapon _returnvalue))
      (return _asbp_weapon))))

(fn GetTotalCost
  (return (+ (.Price (Utilities|Struct|BreakF_VehiclePart_Stats (Variables|Default|GetPart%20Stats))) (Variables|/Script/ExMachinaRemake.Item|GetPrice (Pure|GetWeaponSafe)))))

(fn GetAllItems
  (bind _weaponslot (Variables|Default|GetWeaponSlot))
  (bind _resultitems (LocalVariables|GetResultItems))
  (bind _weapon (Variables|/Script/ExMachinaRemake.WeaponSlot|GetWeapon _weaponslot))
  (Utilities|Array|Clear _resultitems)
  (Utilities|IsValid _weapon
    (:Is%20Valid
      (Utilities|Array|Add _resultitems _weapon))
    (:Is%20Not%20Valid
      _))
  (return _resultitems))

(fn SaveVehiclePart
  (bind _weaponslot (Variables|Default|GetWeaponSlot))
  (bind _part_stats (Variables|Default|GetPart%20Stats))
  (Utilities|IsValid _weaponslot
    (:Is%20Valid
      (if (Class|WeaponSlot|HasWeapon _weaponslot)
        (return (Utilities|Struct|MakeF_SaveGame_VehiclePart _part_stats (Class|Weapon|SaveWeapon (Variables|/Script/ExMachinaRemake.WeaponSlot|GetWeapon _weaponslot))))
        (else
          _)))
    (:Is%20Not%20Valid
      _))
  (return (Utilities|Struct|MakeF_SaveGame_VehiclePart _part_stats "(WeaponStats=(Damage=0,WeaponType=None,DamageType=None,FiringRate=0.000000,FiringRange=0.000000,ChargeSize=0,RecharingTime=0.000000,Durability=0.000000,IsAuto=False,Barrels=,BarrelType=Normal,FireSound=None,TailSound=None,Model=None,DisplayName=\"\",Price=0.000000,Icon=None),CurrentCharge=0,Name=\"\",DisplayName=\"\",Price=0.000000,Icon=None)")))

(fn LoadVehiclePart
  (params (Load :type F%20Save%20Game%20Vehicle%20Part%20Structure))
  (Variables|Default|SetPart%20Stats (.partstats Load))
  (Technical|InitComponents)
  (if (!= (.Name (Utilities|Struct|BreakF_SaveGame_Weapon (.weaponstats Load))) "")
    (bind _returnvalue (Class|CustomFunctionLibrary|CreateObject "/Game/BP_C++/BP_Weapon.BP_Weapon_C"))
    (bind _asbp_weapon (Utilities|Casting|CastToBP_Weapon _returnvalue))
    (Class|Weapon|LoadWeapon _asbp_weapon (.weaponstats Load))
    (Class|WeaponSlot|TrySetWeapon (Variables|Default|GetWeaponSlot) _asbp_weapon)
    (else
      (Class|WeaponSlot|RemoveWeapon (Variables|Default|GetWeaponSlot)))))

(fn HasItem
  (params (Item :type Item%20Object%20Reference))
  (return (== Item (Pure|GetWeapon))))

(fn GetDisplayName
  (return (Utilities|Struct|BreakF_VehiclePart_Stats (Variables|Default|GetPart%20Stats))))

(fn GetIcon
  (return (Utilities|Struct|BreakF_VehiclePart_Stats (Variables|Default|GetPart%20Stats))))

(fn GetPrice
  (return (Utilities|Struct|BreakF_VehiclePart_Stats (Variables|Default|GetPart%20Stats))))