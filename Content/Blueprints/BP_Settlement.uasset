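; BP_Settlement is a trading-post actor where the player buys and sells trade goods and equipment and trades in cabins, cargos and whole cars.
; A data table row seeds its stock on BeginPlay, with random rolls deciding available equipment and vehicle parts.
; Trade-good prices shift multiplicatively with each purchase or sale, and vehicle trade-ins credit half value plus contents.
; Save and load functions persist its stats and all stock.
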(event EventBeginPlay
  (bind _asinventory (CallFunction|CreateSettlementInventory))
  (Variables|Default|SetInventory _asinventory)
  (CallFunction|SetfromTable (Variables|Default|GetRowName)))

(event Collision|EventActorBeginOverlap
  (params (OtherActor :type Actor%20Object%20Reference)))

(event EventTick
  (params (DeltaSeconds :type Float%20%28single-precision%29)))

(fn ConstructionScript)

(fn CheckifPlayerinRange
  (return (Utilities|Array|IsNotEmpty (Collision|GetOverlappingActors (Variables|Default|GetEnterCollision) "/Game/Blueprints/Player/BP_PlayerPawn.BP_PlayerPawn_C" :!class /Script/Engine.PrimitiveComponent))))

(fn SetfromTable
  (params (Name :type Name))
  (bind _returnvalue (Utilities|GetDataTableRow "/Game/Tables/TSettlements.TSettlements" Name)
    (:then
      (Variables|Default|SetStats _returnvalue)
      (CallFunction|ResetWares))))

(fn ResetWares
  (TradeItems|ResetTradeItems)
  (Equipment|ResetEquipment)
  (Cabins|ResetCabins)
  (Cargos|ResetCargos)
  (Cars|ResetCars))

(fn BuyTradeItemfromSettlement
  (params (Name :type Name) (Buyer%20Inventory :type Inventory%20Object%20Reference))
  (bind (_hasdata _data _index) (TradeItems|GetTradeItemData Name))
  (bind _tradeitems (Variables|Default|GetTradeItems))
  (bind (_bexport _currentcount) (Utilities|Struct|BreakF_SettlementGoodsData _data))
  (bind _price (TradeItems|CalculateTradeItemBuyPrice _data))
  (bind _output (Utilities|Array|Get(acopy) _tradeitems _index))
  (bind (_currentmultiplier _currentcount_2) (Utilities|Struct|BreakF_SettlementGoodsData _output))
  (if (Math|Boolean|ANDBoolean _hasdata _bexport (> _currentcount 0) (> (CallFunction|GetPlayerMoney) _price))
    (bind _returnvalue (Class|TradeItem|CreateTradeItemfromTable 0 "/Game/Tables/TTradeItems.TTradeItems" Name))
    (bind _returnvalue_2 (Class|Inventory|TryDropItemInside Buyer%20Inventory _returnvalue))
    (if _returnvalue_2
      (Utilities|Struct|SetmembersinF_SettlementGoodsData _output (* _currentmultiplier 1.05) (- _currentcount_2 1))
      (CallFunction|AddPlayerMoney (CallFunction|NegateInt _price))
      (Default|CallOnTradeItemTransaction Name)
      (return))))

(fn SellTradeItemtoSettlement
  (params (TradeItem :type Trade%20Item%20Object%20Reference) (PriceMultiplier :type Float%20%28double-precision%29))
  (bind _tradeitems (Variables|Default|GetTradeItems))
  (bind _name (Variables|/Script/ExMachinaRemake.Item|GetName TradeItem))
  (bind (_hasdata _data _index) (TradeItems|GetTradeItemData _name))
  (bind _output (Utilities|Array|Get(acopy) _tradeitems _index))
  (bind (_currentmultiplier _currentcount) (Utilities|Struct|BreakF_SettlementGoodsData _output))
  (if _hasdata
    (Utilities|Struct|SetmembersinF_SettlementGoodsData _output (* _currentmultiplier 0.95) (+ _currentcount 1))
    (CallFunction|AddPlayerMoney (TradeItems|CalculateTradeItemSellPrice _data PriceMultiplier))
    (Default|CallOnTradeItemTransaction _name)
    (return true)
    (else
      (return false))))

(fn GetTradeItemData
  (params (Name :type Name))
  (for (_array_element _array_index) (Variables|Default|GetTradeItems)
    (if (== (Utilities|Struct|BreakF_SettlementGoodsData _array_element) Name)
      (return true _array_element _array_index)))
  (return true "" 0))

(fn CalculateTradeItemSellPrice
  (params (Stats :type F%20Settlement%20Goods%20Data%20Structure) (PriceMultiplier :type Float%20%28double-precision%29))
  (bind (_bexport _basepricemultiplier _currentmultiplier _cachedprice) (Utilities|Struct|BreakF_SettlementGoodsData Stats))
  (bind _returnvalue (* _basepricemultiplier _currentmultiplier))
  (bind _returnvalue_2 (* _returnvalue _cachedprice PriceMultiplier))
  (if _bexport
    (return (Math|Float|Round (* _returnvalue_2 0.5)))
    (else
      (return (Math|Float|Round _returnvalue_2)))))

(fn CalculateTradeItemBuyPrice
  (params (Stats :type F%20Settlement%20Goods%20Data%20Structure))
  (bind (_bexport _basepricemultiplier _currentmultiplier _cachedprice) (Utilities|Struct|BreakF_SettlementGoodsData Stats))
  (if _bexport
    (return (Math|Float|Round (* (* _basepricemultiplier _currentmultiplier) _cachedprice)))
    (else
      (return 0))))

(fn SellItemtoSettlement
  (params (Item :type Item%20Object%20Reference) (PriceMultiplier :type Float%20%28double-precision%29))
  (bind _wassold (TradeItems|SellTradeItemtoSettlement (.AsTrade%20Item (Utilities|Casting|CastToTradeItem Item)) PriceMultiplier))
  (return _wassold))

(fn CalculateVehiclePartSellCost
  (params (Vehicle%20Part :type Vehicle%20Part%20Object%20Reference))
  (LocalVariables|SetVehiclePartCost (* (Utilities|Struct|BreakVehiclePartStats (Variables|/Script/ExMachinaRemake.VehiclePart|GetVehiclePartStats Vehicle%20Part)) 0.5))
  (for _array_element (Class|VehiclePart|GetAllItems Vehicle%20Part)
    (LocalVariables|SetVehiclePartCost (+ (LocalVariables|GetVehiclePartCost) (CallFunction|CalculateItemSellPrice _array_element))))
  (return (LocalVariables|GetVehiclePartCost)))

(fn BuyEquipmentfromSettlement
  (params (Item :type Item%20Object%20Reference))
  (CallFunction|AddPlayerMoney (CallFunction|NegateInt (Equipment|CalculateEquipmentBuyPrice Item)))
  (return))

(fn SellEquipmenttoSettlement
  (params (Item :type Item%20Object%20Reference) (PriceMultiplier :type Float%20%28double-precision%29))
  (bind _returnvalue (Class|Inventory|TryDropItemInside (Variables|Default|GetInventory) Item))
  (if _returnvalue
    (CallFunction|AddPlayerMoney (Equipment|CalculateEquipmentSellPrice Item PriceMultiplier))
    (return true)
    (else
      (return false))))

(fn CalculateEquipmentBuyPrice
  (params (Item :type Item%20Object%20Reference))
  (return (Math|Float|Round (* (Variables|/Script/ExMachinaRemake.Item|GetPrice Item) (Utilities|Struct|BreakF_SettlementStats (Variables|Default|GetStats))))))

(fn CalculateEquipmentSellPrice
  (params (Item :type Item%20Object%20Reference) (PriceMultiplier :type Float%20%28double-precision%29))
  (return (Math|Float|Round (* (Variables|/Script/ExMachinaRemake.Item|GetPrice Item) (Utilities|Struct|BreakF_SettlementStats (Variables|Default|GetStats)) PriceMultiplier 0.5))))

(fn ResetTradeItems
  (Utilities|FlowControl|Sequence
    (:then_0
      (Utilities|Array|Clear (Variables|Default|GetTradeItems))
      (bind _outrownames (DataTable|GetDataTableRowNames "/Game/Tables/TTradeItems.TTradeItems"))
      (for _array_element _outrownames
        (bind _returnvalue (Utilities|GetDataTableRow "/Game/Tables/TTradeItems.TTradeItems" _array_element)
          (:then
            (Utilities|Array|Add (Variables|Default|GetTradeItems) (Utilities|Struct|MakeF_SettlementGoodsData _array_element false 0 1.0 1.0 0 (Utilities|Struct|BreakItemStats _returnvalue)))))))
    (:then_1
      (for _array_element_2 (Utilities|Struct|BreakF_SettlementStats (Variables|Default|GetStats))
        (Utilities|Struct|SetmembersinF_SettlementGoodsData (Utilities|Array|Get(acopy) (Variables|Default|GetTradeItems) (.Index (TradeItems|GetTradeItemData (.Name (Utilities|Struct|BreakF_SettlementGoodsData _array_element_2))))) (.bExport (Utilities|Struct|BreakF_SettlementGoodsData _array_element_2)) (.InitialCount (Utilities|Struct|BreakF_SettlementGoodsData _array_element_2)) (.BasePriceMultiplier (Utilities|Struct|BreakF_SettlementGoodsData _array_element_2)) (.InitialCount (Utilities|Struct|BreakF_SettlementGoodsData _array_element_2)))))))

(fn ResetEquipment
  (bind _inventory (Variables|Default|GetInventory))
  (Class|Inventory|Clear (Variables|Default|GetInventory))
  (for _array_element (Utilities|Struct|BreakF_SettlementStats (Variables|Default|GetStats))
    (if (Math|Random|RandomBoolwithWeight (.AvailabilityProbability (Utilities|Struct|BreakF_SettlementGeneralData _array_element)))
      (switch Utilities|FlowControl|Switch|SwitchonEItemType (.ItemType (Utilities|Struct|BreakF_SettlementGeneralData _array_element))
        (:Weapon
          (bind _result (CallFunction|CreateWeaponfromTable (.Name (Utilities|Struct|BreakF_SettlementGeneralData _array_element))))
          (Class|Inventory|TryDropItemInside _inventory _result))
        (:GadgetCommon
          (bind _result_2 (CallFunction|CreateGadgetCommonfromTable (.Name (Utilities|Struct|BreakF_SettlementGeneralData _array_element))))
          (Class|Inventory|TryDropItemInside _inventory _result_2))
        (:GadgetWeapon
          (bind _result_3 (CallFunction|CreateGadgetWeaponfromTable (.Name (Utilities|Struct|BreakF_SettlementGeneralData _array_element))))
          (Class|Inventory|TryDropItemInside _inventory _result_3))))))

(fn ResetCabins
  (Utilities|Array|Clear (Variables|Default|GetCabins))
  (for _array_element (Utilities|Struct|BreakF_SettlementStats (Variables|Default|GetStats))
    (if (Math|Random|RandomBoolwithWeight (.availabilityprobability _array_element))
      (bind _returnvalue (Class|CustomFunctionLibrary|CreateObject "/Script/ExMachinaRemake.Cabin"))
      (Class|VehiclePart|SetfromTable (.AsCabin (Utilities|Casting|CastToCabin _returnvalue)) "/Game/Tables/TCabins.TCabins" (.name _array_element))
      (Utilities|Array|Add (Variables|Default|GetCabins) (.AsCabin (Utilities|Casting|CastToCabin _returnvalue))))))

(fn GetCabinsforCar
  (params (Car :type Name))
  (bind _resultcabins (LocalVariables|GetResultCabins))
  (Utilities|Array|Clear _resultcabins)
  (for _array_element (Variables|Default|GetCabins)
    (if (== (Utilities|Struct|BreakVehiclePartStats (Variables|/Script/ExMachinaRemake.VehiclePart|GetVehiclePartStats _array_element)) Car)
      (Utilities|Array|Add (LocalVariables|GetResultCabins) _array_element)))
  (return _resultcabins))

(fn TryTradeCabins
  (params (SourceVehicle :type BP%20Vehicle%20Pawn%20Object%20Reference) (New%20Cabin :type Cabin%20Object%20Reference) (New%20Cargo :type Cargo%20Object%20Reference) (Old%20Cabin%20To%20Sell :type Cabin%20Object%20Reference) (New%20Cabin%20Market%20Ref :type Cabin%20Object%20Reference))
  (bind _cost (CallFunction|CalculateVehiclePartSellCost Old%20Cabin%20To%20Sell))
  (bind _vehiclepartstats (Variables|/Script/ExMachinaRemake.VehiclePart|GetVehiclePartStats New%20Cabin))
  (bind _cabins (Variables|Default|GetCabins))
  (bind _price (Utilities|Struct|BreakVehiclePartStats _vehiclepartstats))
  (bind _returnvalue (- _price _cost))
  (bind _returnvalue_2 (Math|Float|Round _returnvalue))
  (if (>= (CallFunction|GetPlayerMoney) _returnvalue_2)
    (CallFunction|AddPlayerMoney (CallFunction|NegateInt _returnvalue_2))
    (Class|VehiclePart|Copyto New%20Cabin (Variables|/Game/Blueprints/Vehicle/BP_VehiclePawn.BP_VehiclePawn_C|GetCabin SourceVehicle))
    (Class|VehiclePart|Copyto New%20Cargo (Variables|/Game/Blueprints/Vehicle/BP_VehiclePawn.BP_VehiclePawn_C|GetCargo SourceVehicle))
    (Default|BindCabinComponent SourceVehicle)
    (Utilities|Array|RemoveItem _cabins New%20Cabin%20Market%20Ref)
    (Utilities|Array|Add _cabins Old%20Cabin%20To%20Sell)
    (CallFunction|SellAllVehiclePartItems Old%20Cabin%20To%20Sell 0.0)
    (return true)
    (else
      (return false))))

(fn ResetCargos
  (Utilities|Array|Clear (Variables|Default|GetCargos))
  (for _array_element (Utilities|Struct|BreakF_SettlementStats (Variables|Default|GetStats))
    (if (Math|Random|RandomBoolwithWeight (.availabilityprobability _array_element))
      (bind _returnvalue (Class|CustomFunctionLibrary|CreateObject "/Script/ExMachinaRemake.Cargo"))
      (Class|Cargo|SetfromTable (.AsCargo (Utilities|Casting|CastToCargo _returnvalue)) "/Game/Tables/TCargos.TCargos" (.name _array_element))
      (Utilities|Array|Add (Variables|Default|GetCargos) (.AsCargo (Utilities|Casting|CastToCargo _returnvalue))))))

(fn GetCargosforCar
  (params (Car :type Name))
  (Utilities|Array|Clear (LocalVariables|GetResultCargos))
  (for _array_element (Variables|Default|GetCargos)
    (if (== (Utilities|Struct|BreakVehiclePartStats (Variables|/Script/ExMachinaRemake.VehiclePart|GetVehiclePartStats _array_element)) Car)
      (Utilities|Array|Add (LocalVariables|GetResultCargos) _array_element)))
  (return (LocalVariables|GetResultCargos)))

(fn TryTradeCargos
  (params (SourceVehicle :type BP%20Vehicle%20Pawn%20Object%20Reference) (New%20Cabin :type Cabin%20Object%20Reference) (New%20Cargo :type Cargo%20Object%20Reference) (Old%20Cargo%20To%20Sell :type Cargo%20Object%20Reference) (New%20Cargo%20%20Market%20Ref :type Cargo%20Object%20Reference))
  (bind _cost (CallFunction|CalculateVehiclePartSellCost Old%20Cargo%20To%20Sell))
  (bind _vehiclepartstats (Variables|/Script/ExMachinaRemake.VehiclePart|GetVehiclePartStats New%20Cabin))
  (bind _cargos (Variables|Default|GetCargos))
  (bind _price (Utilities|Struct|BreakVehiclePartStats _vehiclepartstats))
  (bind _returnvalue (- _price _cost))
  (bind _returnvalue_2 (Math|Float|Round _returnvalue))
  (if (>= (CallFunction|GetPlayerMoney) _returnvalue_2)
    (CallFunction|AddPlayerMoney (CallFunction|NegateInt _returnvalue_2))
    (Class|VehiclePart|Copyto New%20Cabin (Variables|/Game/Blueprints/Vehicle/BP_VehiclePawn.BP_VehiclePawn_C|GetCabin SourceVehicle))
    (Class|VehiclePart|Copyto New%20Cargo (Variables|/Game/Blueprints/Vehicle/BP_VehiclePawn.BP_VehiclePawn_C|GetCargo SourceVehicle))
    (Default|BindCargoComponent SourceVehicle)
    (Utilities|Array|RemoveItem _cargos New%20Cargo%20%20Market%20Ref)
    (Utilities|Array|Add _cargos Old%20Cargo%20To%20Sell)
    (CallFunction|SellAllVehiclePartItems Old%20Cargo%20To%20Sell 0.0)
    (return true)
    (else
      (return false))))

(fn CalculateItemSellPrice
  (params (Item :type Item%20Object%20Reference))
  (bind _astrade_item (Utilities|Casting|CastToTradeItem Item)
    (:then
      (return (TradeItems|CalculateTradeItemSellPrice (.Data (TradeItems|GetTradeItemData (Variables|/Script/ExMachinaRemake.Item|GetName _astrade_item))) 1.0)))
    (:CastFailed
      (return (Equipment|CalculateEquipmentSellPrice Item 1.0)))))

(fn ResetCars
  (Utilities|Array|Clear (Variables|Default|GetCars))
  (for _array_element (Utilities|Struct|BreakF_SettlementStats (Variables|Default|GetStats))
    (bind _returnvalue (Class|CustomFunctionLibrary|CreateObject "/Game/Blueprints/Vehicle/BP_VehiclePawn.BP_VehiclePawn_C"))
    (bind _asbp_vehicle_pawn (Utilities|Casting|CastToBP_VehiclePawn _returnvalue))
    (Default|AddFakeComponents _asbp_vehicle_pawn)
    (Default|SetCar _asbp_vehicle_pawn _array_element true)
    (Utilities|Array|Add (Variables|Default|GetCars) _asbp_vehicle_pawn)))

(fn TryTradeCars
  (params (SourceVehicle :type BP%20Vehicle%20Pawn%20Object%20Reference) (MarketVehicle :type BP%20Vehicle%20Pawn%20Object%20Reference) (Source%20Cabin :type Cabin%20Object%20Reference) (Source%20Cargo :type Cargo%20Object%20Reference) (Market%20Cabin :type Cabin%20Object%20Reference) (Market%20Cargo :type Cargo%20Object%20Reference))
  (bind _cost (CallFunction|CalculateVehiclePartSellCost Source%20Cargo))
  (bind _cost_2 (CallFunction|CalculateVehiclePartSellCost Source%20Cabin))
  (bind _vehiclepartstats (Variables|/Script/ExMachinaRemake.VehiclePart|GetVehiclePartStats Market%20Cabin))
  (bind _vehiclepartstats_2 (Variables|/Script/ExMachinaRemake.VehiclePart|GetVehiclePartStats Market%20Cargo))
  (bind _stats (Variables|/Game/Blueprints/Vehicle/BP_VehiclePawn.BP_VehiclePawn_C|GetStats MarketVehicle))
  (bind _stats_2 (Variables|/Game/Blueprints/Vehicle/BP_VehiclePawn.BP_VehiclePawn_C|GetStats SourceVehicle))
  (bind _price (Utilities|Struct|BreakF_Car_Stats _stats))
  (bind _price_2 (Utilities|Struct|BreakF_Car_Stats _stats_2))
  (bind _price_3 (Utilities|Struct|BreakVehiclePartStats _vehiclepartstats))
  (bind _price_4 (Utilities|Struct|BreakVehiclePartStats _vehiclepartstats_2))
  (bind _cabin (Variables|/Game/Blueprints/Vehicle/BP_VehiclePawn.BP_VehiclePawn_C|GetCabin MarketVehicle))
  (bind _cargo (Variables|/Game/Blueprints/Vehicle/BP_VehiclePawn.BP_VehiclePawn_C|GetCargo MarketVehicle))
  (bind _returnvalue (+ _price_3 _price_4 _price))
  (bind _returnvalue_2 (* _price_2 0.5))
  (bind _returnvalue_3 (+ _cost_2 _cost _returnvalue_2))
  (bind _returnvalue_4 (- _returnvalue _returnvalue_3))
  (bind _returnvalue_5 (Math|Float|Round _returnvalue_4))
  (LocalVariables|SetSourceCarName (Variables|/Game/Blueprints/Vehicle/BP_VehiclePawn.BP_VehiclePawn_C|GetCarName SourceVehicle))
  (if (>= (CallFunction|GetPlayerMoney) _returnvalue_5)
    (CallFunction|AddPlayerMoney (CallFunction|NegateInt _returnvalue_5))
    (Default|SetCar SourceVehicle (Variables|/Game/Blueprints/Vehicle/BP_VehiclePawn.BP_VehiclePawn_C|GetCarName MarketVehicle) false)
    (Class|VehiclePart|Copyto Market%20Cabin (Variables|/Game/Blueprints/Vehicle/BP_VehiclePawn.BP_VehiclePawn_C|GetCabin SourceVehicle))
    (Class|VehiclePart|Copyto Market%20Cargo (Variables|/Game/Blueprints/Vehicle/BP_VehiclePawn.BP_VehiclePawn_C|GetCargo SourceVehicle))
    (Default|SetCar MarketVehicle (LocalVariables|GetSourceCarName) false)
    (Class|VehiclePart|Copyto Source%20Cabin _cabin)
    (Class|VehiclePart|Copyto Source%20Cargo _cargo)
    (Default|BindCabinComponent SourceVehicle)
    (Default|BindCargoComponent SourceVehicle)
    (CallFunction|SellAllVehiclePartItems _cabin 0.0)
    (CallFunction|SellAllVehiclePartItems _cargo 0.0)
    (return true)
    (else
      (return false))))

(fn SaveSettlement
  (for _array_element (Variables|Default|GetCabins)
    (Utilities|Array|Add (LocalVariables|GetSaveCabins) (Class|Cabin|SaveCabin _array_element)))
  (for _array_element_2 (Variables|Default|GetCargos)
    (Utilities|Array|Add (LocalVariables|GetSaveCargos) (Class|Cargo|SaveCargo _array_element_2)))
  (for _array_element_3 (Variables|Default|GetCars)
    (Utilities|Array|Add (LocalVariables|GetSaveCars) (Default|SaveVehiclePawn _array_element_3)))
  (return (Utilities|Struct|MakeF_SaveGame_Settlement (Variables|Default|GetRowName) (Variables|Default|GetId) (Variables|Default|GetStats) (Class|Inventory|SaveInventory (Variables|Default|GetInventory)) (Variables|Default|GetTradeItems) (LocalVariables|GetSaveCabins) (LocalVariables|GetSaveCargos) (LocalVariables|GetSaveCars))))

(fn LoadSettlement
  (params (Load :type F%20Save%20Game%20Settlement%20Structure))
  (bind _cabins (Variables|Default|GetCabins))
  (bind _cargos (Variables|Default|GetCargos))
  (bind _cars (Variables|Default|GetCars))
  (Variables|Default|SetRowName (.rowname Load))
  (Variables|Default|SetStats (.stats Load))
  (Variables|Default|SetTradeItems (.tradeitems Load))
  (bind _returnvalue (Class|CustomFunctionLibrary|CreateObject "/Script/ExMachinaRemake.Inventory"))
  (bind _output_get (Variables|Default|SetInventory (.AsInventory (Utilities|Casting|CastToInventory _returnvalue))))
  (Class|Inventory|LoadInventory _output_get (.inventory Load))
  (Utilities|Array|Clear _cabins)
  (for _array_element (.cabins Load)
    (bind _returnvalue_2 (Class|CustomFunctionLibrary|CreateObject "/Script/ExMachinaRemake.Cabin"))
    (Class|Cabin|LoadCabin (.AsCabin (Utilities|Casting|CastToCabin _returnvalue_2)) _array_element)
    (Utilities|Array|Add _cabins 0))
  (Utilities|Array|Clear _cargos)
  (for _array_element_2 (.cargos Load)
    (bind _returnvalue_3 (Class|CustomFunctionLibrary|CreateObject "/Script/ExMachinaRemake.Cargo"))
    (Class|Cargo|LoadCargo (.AsCargo (Utilities|Casting|CastToCargo _returnvalue_3)) _array_element_2)
    (Utilities|Array|Add _cargos 0))
  (Utilities|Array|Clear _cars)
  (for _array_element_3 (.cars Load)
    (bind _returnvalue_4 (Class|CustomFunctionLibrary|CreateObject "/Game/Blueprints/Vehicle/BP_VehiclePawn.BP_VehiclePawn_C"))
    (Default|AddFakeComponents (.AsBP%20Vehicle%20Pawn (Utilities|Casting|CastToBP_VehiclePawn _returnvalue_4)))
    (Default|LoadVehiclePawn (.AsBP%20Vehicle%20Pawn (Utilities|Casting|CastToBP_VehiclePawn _returnvalue_4)) _array_element_3)
    (Utilities|Array|Add _cars (.AsBP%20Vehicle%20Pawn (Utilities|Casting|CastToBP_VehiclePawn _returnvalue_4)))))

(fn SellAllVehiclePartItems
  (params (Vehicle%20Part :type Vehicle%20Part%20Object%20Reference) (Price%20Multiplier :type Float%20%28double-precision%29))
  (for _array_element (Class|VehiclePart|GetAllItems Vehicle%20Part)
    (CallFunction|SellItemtoSettlement _array_element Price%20Multiplier))
  (Class|VehiclePart|RemoveAllItems Vehicle%20Part))