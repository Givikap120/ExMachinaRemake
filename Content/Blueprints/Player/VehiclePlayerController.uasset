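; Player controller for the vehicle pawn, handling the in-game menu and quick save/load on F5/F9 to an AutoSave slot.
; BeginPlay caches the BP_PlayerPawn and creates one reusable UI_GeneralMenu widget.
; Input actions open it as travel inventory or for the first BP_Settlement reporting the player in range.
; ToggleMenu uses pause state to show or hide the menu, switching cursor and input mode, unless the player is dead.
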(event Input|EnhancedActionEvents|EnhancedInputActionIA_EnterSettlement
  (params (ActionValue :type Boolean) (ElapsedSeconds :type Float%20%28double-precision%29) (TriggeredSeconds :type Float%20%28double-precision%29) (InputAction :type Input%20Action%20Object%20Reference :default "/Game/Input/Actions/IA_EnterSettlement.IA_EnterSettlement"))
  (:Started
    (bind _outactors (Actor|GetAllActorsOfClass "/Game/Blueprints/BP_Settlement.BP_Settlement_C"))
    (bind _array_element (Utilities|Array|ForEachLoopwithBreak _outactors :!label _label)
      (:LoopBody
        (bind _return_value (Default|CheckifPlayerinRange _array_element))
        (if _return_value
          (Default|InitforSettlement (Variables|Default|GetGeneralMenu) _array_element)
          (CallFunction|ToggleMenu)
          (goto _label Break))))))

(event Input|EnhancedActionEvents|EnhancedInputActionIA_OpenInventory
  (params (ActionValue :type Boolean) (ElapsedSeconds :type Float%20%28double-precision%29) (TriggeredSeconds :type Float%20%28double-precision%29) (InputAction :type Input%20Action%20Object%20Reference :default "/Game/Input/Actions/IA_OpenInventory.IA_OpenInventory"))
  (:Started
    (CallFunction|ToggleMenu)
    (Default|InitforTravelInventory (Variables|Default|GetGeneralMenu))))

(event EventBeginPlay
  (bind _asbp_player_pawn (Utilities|Casting|CastToBP_PlayerPawn (Pawn|GetControlledPawn)))
  (Variables|Default|SetParent _asbp_player_pawn)
  (Variables|Default|SetVehicle%20Movement%20Component (Variables|/Script/ChaosVehicles.WheeledVehiclePawn|GetVehicleMovementComponent _asbp_player_pawn))
  (bind _returnvalue (UserInterface|CreateWidget "/Game/UI/GeneralMenu/UI_GeneralMenu.UI_GeneralMenu_C" 0 (Variables|Default|GetParent)))
  (Variables|Default|SetGeneralMenu _returnvalue))

(event Input|KeyboardEvents|F5
  (params (Key :type Key%20Structure))
  (:Pressed
    (CallFunction|SaveGame "AutoSave")))

(event Input|KeyboardEvents|F9
  (params (Key :type Key%20Structure))
  (:Pressed
    (CallFunction|LoadGame "AutoSave")))

(fn ConstructionScript)

(fn ToggleMenu
  (bind _returnvalue (Game|GetPlayerController 0))
  (bind _returnvalue_2 (Game|GetPlayerController 0))
  (bind _generalmenu (Variables|Default|GetGeneralMenu))
  (if (not (Variables|/Game/Blueprints/Vehicle/BP_VehiclePawn.BP_VehiclePawn_C|GetbDead (Variables|Default|GetParent)))
    (Utilities|IsValid (Variables|Default|GetGeneralMenu)
      (:Is%20Valid
        (if (Game|IsGamePaused)
          (Game|SetGamePaused false)
          (Default|HandleClosing _generalmenu)
          (Widget|RemovefromParent _generalmenu)
          (Variables|/Script/Engine.PlayerController|SetbShowMouseCursor _returnvalue_2 false)
          (Input|SetInputModeGameOnly _returnvalue_2 false)
          (else
            (UserInterface|Viewport|AddtoViewport (Variables|Default|GetGeneralMenu) 0)
            (Game|SetGamePaused true)
            (Variables|/Script/Engine.PlayerController|SetbShowMouseCursor _returnvalue true)
            (Input|SetInputModeUIOnly _returnvalue (Variables|Default|GetGeneralMenu) "DoNotLock" true)))))))