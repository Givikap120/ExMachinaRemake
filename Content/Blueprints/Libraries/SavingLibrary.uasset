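; Blueprint library that saves and loads named game slots through BP_SaveGame.
; Saving captures the player vehicle, camera, money, AI vehicles and settlements.
; Loading restores the player, destroys and respawns AI vehicles from saved data, and updates existing settlements matched by Id.
; Outside ExMachinaGameMode, LoadGame only stores the slot as PendingSaveGame on the game instance.
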(fn SaveGame
  (params (Slot :type String))
  (bind _returnvalue (SaveGame|CreateSaveGameObject "/Game/Blueprints/BP_SaveGame.BP_SaveGame_C"))
  (SaveGame|SaveGametoData _returnvalue)
  (bind _returnvalue_2 (SaveGame|SaveGametoSlot _returnvalue Slot))
  (if _returnvalue_2
    (Development|PrintString 0 "Gave Saved")))

(fn LoadGame
  (params (Slot :type String))
  (Utilities|Casting|CastToExMachinaGameMode (Game|GetGameMode)
    (:then
      (bind _returnvalue (SaveGame|LoadGamefromSlot Slot))
      (bind _asbp_save_game (Utilities|Casting|CastToBP_SaveGame _returnvalue))
      (SaveGame|LoadGamefromData _asbp_save_game)
      (Development|PrintString 0 "Game Loaded"))
    (:CastFailed
      (bind _asex_machina_game_instance (Utilities|Casting|CastToExMachinaGameInstance (Game|GetGameInstance)))
      (Variables|/Game/GameModes/ExMachinaGameInstance.ExMachinaGameInstance_C|SetPendingSaveGame _asex_machina_game_instance Slot))))

(fn SaveGametoData
  (params (Data :type BP%20Save%20Game%20Object%20Reference))
  (bind _vehicles (Variables|/Game/Blueprints/BP_SaveGame.BP_SaveGame_C|GetVehicles Data))
  (bind _settlements (Variables|/Game/Blueprints/BP_SaveGame.BP_SaveGame_C|GetSettlements Data))
  (bind _asbp_player_pawn (Utilities|Casting|CastToBP_PlayerPawn (Game|Player|GetPlayerPawn 0)))
  (Variables|/Game/Blueprints/BP_SaveGame.BP_SaveGame_C|SetPlayerVehicle Data (Default|SaveVehiclePawn _asbp_player_pawn))
  (|SetBy-RefVar (Variables|/Game/Blueprints/BP_SaveGame.BP_SaveGame_C|GetGeneralData Data) (Utilities|Struct|MakeF_GeneralGame_PlayerData (CallFunction|GetPlayerMoney) (Transformation|GetRelativeTransform (Variables|/Game/Blueprints/Player/BP_PlayerPawn.BP_PlayerPawn_C|GetBackCamera _asbp_player_pawn))))
  (Utilities|Array|Clear _vehicles)
  (bind _outactors (Actor|GetAllActorsOfClass 0 "/Game/Blueprints/AI/BP_AIVehiclePawn.BP_AIVehiclePawn_C"))
  (for _array_element _outactors
    (Utilities|Array|Add _vehicles (Default|SaveVehiclePawn _array_element)))
  (Utilities|Array|Clear _settlements)
  (bind _outactors_2 (Actor|GetAllActorsOfClass 0 "/Game/Blueprints/BP_Settlement.BP_Settlement_C"))
  (for _array_element_2 _outactors_2
    (Utilities|Array|Add _settlements (Default|SaveSettlement _array_element_2))))

(fn LoadGamefromData
  (params (Data :type BP%20Save%20Game%20Object%20Reference))
  (bind _generaldata (Variables|/Game/Blueprints/BP_SaveGame.BP_SaveGame_C|GetGeneralData Data))
  (bind _asbp_player_pawn (Utilities|Casting|CastToBP_PlayerPawn (Game|Player|GetPlayerPawn 0)))
  (Default|LoadVehiclePawn _asbp_player_pawn (Variables|/Game/Blueprints/BP_SaveGame.BP_SaveGame_C|GetPlayerVehicle Data))
  (Transformation|SetRelativeTransform (Variables|/Game/Blueprints/Player/BP_PlayerPawn.BP_PlayerPawn_C|GetBackCamera _asbp_player_pawn) (.playercamerapos _generaldata) false true)
  (CallFunction|SetPlayerMoney (.playermoney _generaldata))
  (Utilities|Struct|SetmembersinF_VehiclePreset (Variables|/Game/Blueprints/Vehicle/BP_VehiclePawn.BP_VehiclePawn_C|GetPreset _asbp_player_pawn) false)
  (bind _outactors (Actor|GetAllActorsOfClass 0 "/Game/Blueprints/AI/BP_AIVehiclePawn.BP_AIVehiclePawn_C"))
  (for _array_element _outactors
    (Actor|DestroyActor _array_element))
  (bind _asex_machina_game_mode (Utilities|Casting|CastToExMachinaGameMode (Game|GetGameMode)))
  (for _array_element_2 (Variables|/Game/Blueprints/BP_SaveGame.BP_SaveGame_C|GetVehicles Data)
    (bind _returnvalue (Default|SpawnActor _asex_machina_game_mode "/Game/Blueprints/AI/BP_AIVehiclePawn.BP_AIVehiclePawn_C" (.Transform (Utilities|Struct|BreakF_SaveGame_VehiclePawn _array_element_2)) "AlwaysSpawn"))
    (bind _asbp_aivehicle_pawn (Utilities|Casting|CastToBP_AIVehiclePawn _returnvalue))
    (Default|LoadVehiclePawn _asbp_aivehicle_pawn _array_element_2))
  (bind _outactors_2 (Actor|GetAllActorsOfClass 0 "/Game/Blueprints/BP_Settlement.BP_Settlement_C"))
  (for _array_element_3 _outactors_2
    (bind _data (Private|FindSettlementSaveData (Variables|/Game/Blueprints/BP_Settlement.BP_Settlement_C|GetId _array_element_3) (Variables|/Game/Blueprints/BP_SaveGame.BP_SaveGame_C|GetSettlements Data)))
    (Default|LoadSettlement _array_element_3 _data)))

(fn FormatSaveFileName
  (params (FilePath :type String))
  (return (Utilities|String|LeftChop FilePath 4)))

(fn FindSettlementSaveData
  (params (Id :type Integer) (AllData :type Array%20of%20F%20Save%20Game%20Settlement%20Structures))
  (for _array_element AllData
    (if (== (.Id (Utilities|Struct|BreakF_SaveGame_Settlement _array_element)) Id)
      (return _array_element)))
  (return ""))