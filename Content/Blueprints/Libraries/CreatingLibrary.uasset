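; Blueprint function library for creating game items and inventories.
; Four functions build a Weapon, TradeItem, GadgetWeapon or GadgetCommon from a row name, each pairing its class with a matching data table.
; A separate function creates an Inventory object with a fixed grid capacity for settlements.
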(fn CreateWeaponfromTable
  (params (Name :type Name))
  (bind _returnvalue (Class|Weapon|CreateWeaponfromTable "/Script/ExMachinaRemake.Weapon" "/Game/Tables/TWeapons.TWeapons" Name))
  (return _returnvalue))

(fn CreateTradeItemfromTable
  (params (Name :type Name))
  (bind _returnvalue (Class|TradeItem|CreateTradeItemfromTable "/Script/ExMachinaRemake.TradeItem" "/Game/Tables/TTradeItems.TTradeItems" Name))
  (return _returnvalue))

(fn CreateGadgetWeaponfromTable
  (params (Name :type Name))
  (bind _returnvalue (Class|GadgetWeapon|CreateGadgetWeaponfromTable "/Script/ExMachinaRemake.GadgetWeapon" "/Game/Tables/TGadgetsWeapon.TGadgetsWeapon" Name))
  (return _returnvalue))

(fn CreateGadgetCommonfromTable
  (params (Name :type Name))
  (bind _returnvalue (Class|GadgetCommon|CreateGadgetCommonfromTable "/Script/ExMachinaRemake.GadgetCommon" "/Game/Tables/TGadgetsCommon.TGadgetsCommon" Name))
  (return _returnvalue))

(fn CreateSettlementInventory
  (bind _returnvalue (Class|CustomFunctionLibrary|CreateObject "/Script/ExMachinaRemake.Inventory"))
  (bind _asinventory (Utilities|Casting|CastToInventory _returnvalue))
  (Variables|/Script/ExMachinaRemake.Inventory|SetCapacityX _asinventory 12)
  (Variables|/Script/ExMachinaRemake.Inventory|SetCapacityY _asinventory 10)
  (return _asinventory))