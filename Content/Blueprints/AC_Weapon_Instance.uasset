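; Weapon instance component that handles a mounted gun's shoot and reload input and plays its firing sound and animation.
; Enhanced Input actions start and stop shooting or start a reload.
; Visual events play looping or one-shot audio, add a tail sound when a loop stops, and drive the skeletal mesh's BP_WeaponAnimation_Base.
; RotateGunMesh forwards yaw and pitch, while RotateGun ignores its aim inputs and sets zero rotation.
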(event Input|EnhancedActionEvents|EnhancedInputActionIA_Shoot
  (params (ActionValue :type Boolean) (ElapsedSeconds :type Float%20%28double-precision%29) (TriggeredSeconds :type Float%20%28double-precision%29) (InputAction :type Input%20Action%20Object%20Reference :default "/Game/Input/Actions/IA_Shoot.IA_Shoot"))
  (:Started
    (Class|WeaponInstance|TryStartShooting))
  (:Completed
    (Class|WeaponInstance|TryStopShooting)))

(event Input|EnhancedActionEvents|EnhancedInputActionIA_Reload
  (params (ActionValue :type Boolean) (ElapsedSeconds :type Float%20%28double-precision%29) (TriggeredSeconds :type Float%20%28double-precision%29) (InputAction :type Input%20Action%20Object%20Reference :default "/Game/Input/Actions/IA_Reload.IA_Reload"))
  (Class|WeaponInstance|StartReload))

(event EventVisualsEndLoop
  (bind _audiocomponent (Variables|Default|GetAudioComponent))
  (if (Audio|Components|Audio|IsPlaying _audiocomponent)
    (Audio|PlaySoundatLocation (Variables|/Script/ExMachinaRemake.Weapon|GetTailSound (Variables|Default|GetWeapon)) (Transformation|GetWorldLocation (Variables|Default|GetSkeletalMeshComponent)) "0, 0, 0" 1.0 1.0 0.0 "/Game/Blueprints/LocalAttenuation.LocalAttenuation" 0 0 0))
  (Audio|Components|Audio|Stop _audiocomponent)
  (bind _asbp_weapon_animation_base (Utilities|Casting|CastToBP_WeaponAnimation_Base (Components|SkeletalMesh|GetAnimInstance (Variables|Default|GetSkeletalMeshComponent))))
  (Default|StopShooting _asbp_weapon_animation_base))

(event EventVisualsPlayOnce
  (bind _skeletalmeshcomponent (Variables|Default|GetSkeletalMeshComponent))
  (Audio|PlaySoundatLocation (Variables|/Script/Engine.AudioComponent|GetSound (Variables|Default|GetAudioComponent)) (Transformation|GetWorldLocation _skeletalmeshcomponent) "0, 0, 0" 1.0 1.0 0.0 "/Game/Blueprints/LocalAttenuation.LocalAttenuation" 0 0 0)
  (bind _asbp_weapon_animation_base (Utilities|Casting|CastToBP_WeaponAnimation_Base (Components|SkeletalMesh|GetAnimInstance _skeletalmeshcomponent))
    (:then
      (Default|ShootOnce _asbp_weapon_animation_base))
    (:CastFailed
      (Development|PrintString "ERROR in animation casting"))))

(event EventVisualsStartLoop
  (Audio|Components|Audio|Play (Variables|Default|GetAudioComponent) 0.0)
  (bind _asbp_weapon_animation_base (Utilities|Casting|CastToBP_WeaponAnimation_Base (Components|SkeletalMesh|GetAnimInstance (Variables|Default|GetSkeletalMeshComponent)))
    (:then
      (Default|StartShooting _asbp_weapon_animation_base))
    (:CastFailed
      (Development|PrintString "ERROR in animation casting"))))

(event EventRotateGunMesh
  (params (Yaw :type Float%20%28single-precision%29) (Pitch :type Float%20%28single-precision%29))
  (bind _asbp_weapon_animation_base (Utilities|Casting|CastToBP_WeaponAnimation_Base (Components|SkeletalMesh|GetAnimInstance (Variables|Default|GetSkeletalMeshComponent))))
  (Default|SetGunRotaton _asbp_weapon_animation_base Yaw Pitch))

(fn RotateGun
  (params (AimPoint :type Vector) (CarRotation :type Rotator))
  (bind _asbp_weapon_animation_base (Utilities|Casting|CastToBP_WeaponAnimation_Base (Components|SkeletalMesh|GetAnimInstance (Variables|Default|GetSkeletalMeshComponent))))
  (Default|SetGunRotaton _asbp_weapon_animation_base 0.0 0.0))