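; Enemy spawn system that periodically spawns AI vehicle groups near the player outside safe zones.
; A looping timer rolls a probability scaled by living enemy count, then picks the nearest eligible spawn point within a distance band.
; Random car, cabin, cargo and weapon presets share budgets from player cost and max HP, filtered by minimum costs precomputed from DataTables.
; Vehicles spawn in a ring, retrying higher when blocked, and head for the player's position.
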(event Custom|TrySpawnEnemies
  (bind _asex_machina_game_mode (Utilities|Casting|CastToExMachinaGameMode (Game|GetGameMode)))
  (if (Variables|/Game/GameModes/ExMachinaGameMode.ExMachinaGameMode_C|GetbPlayerInSafeZone _asex_machina_game_mode)
    (Utilities|DebugOnly
      (:DebugOnly
        (Development|PrintString "NO SPAWN: player is in safe zone")))
    (else
      (bind (_was_successful _probability_debug) (CallFunction|CheckSpawnProbability))
      (if _was_successful
        (bind (_was_successful_2 _point) (CallFunction|FindSpawnPoint))
        (if _was_successful_2
          (bind _enemypresets (CallFunction|CalculateEnemyPresets))
          (bind _output_get (Variables|Private|SetWasSpawned 0))
          (for (_array_element _array_index) _enemypresets
            (bind _result (CallFunction|GetSpawnPosition (Transformation|GetActorLocation _point) (Variables|/Game/Blueprints/EnemySpawn/BP_EnemySpawnPoint.BP_EnemySpawnPoint_C|GetSpawnRadius _point) _array_index (Math|Float|SafeDivide (Math|Float|MultiplybyPi 2.0) (Math|Conversions|ToFloat(Integer) (Utilities|Array|Length _enemypresets)))))
            (bind _wasspawned (CallFunction|TrySpawnat _result _array_element))
            (if _wasspawned
              (Math|Integer|IncrementInt (Variables|Private|GetWasSpawned))))
          (if (> _output_get 0)
            (Math|Integer|IncrementInt (Variables|/Game/Blueprints/EnemySpawn/BP_EnemySpawnPoint.BP_EnemySpawnPoint_C|GetSpawnCount _point)
              (:%20%20
                _)))
          (Utilities|DebugOnly
            (:DebugOnly
              (Development|PrintString (Utilities|String|Append "SPAWN (" (Utilities|String|ToString(Integer) (Variables|Private|GetWasSpawned)) "/" (Utilities|String|ToString(Integer) (Utilities|Array|Length _enemypresets)) "): p = " _probability_debug))))
          (else
            (Utilities|DebugOnly
              (:DebugOnly
                (Development|PrintString (Utilities|String|Append "NO SPAWN: no acceptable spawn point found, p = " _probability_debug))))))
        (else
          (Utilities|DebugOnly
            (:DebugOnly
              (Development|PrintString (Utilities|String|Append "NO SPAWN: probability failed, p = " _probability_debug)))))))))

(event EventBeginPlay
  (bind _spawndelay (Variables|SpawnParameters|GetSpawnDelay))
  (Utilities|Time|SetTimerbyEvent (delegate Custom|TrySpawnEnemies) _spawndelay true true _spawndelay)
  (CallFunction|PrecalculateMinimalCosts))

(event Collision|EventActorBeginOverlap
  (params (OtherActor :type Actor%20Object%20Reference)))

(event EventTick
  (params (DeltaSeconds :type Float%20%28single-precision%29)))

(event EventEndPlay
  (params (EndPlayReason :type EEndPlayReason%20Enum :default "Destroyed"))
  (Utilities|Time|InvalidateTimerHandle (Variables|Private|GetTimerHandle)))

(fn ConstructionScript)

(fn PrecalculateMinimalCosts
  (bind _minimal_weapon_cost (Variables|Private|GetMinimal%20Weapon%20Cost))
  (bind _minimal_cabin_costs (Variables|Private|GetMinimal%20Cabin%20Costs))
  (bind _minimal_cargo_costs (Variables|Private|GetMinimal%20Cargo%20Costs))
  (Utilities|FlowControl|Sequence
    (:then_0
      (Utilities|Map|Clear (Variables|Private|GetMinimal%20Weapon%20Cost))
      (bind _outrownames (DataTable|GetDataTableRowNames "/Game/Tables/TWeapons.TWeapons"))
      (for _array_element _outrownames
        (bind _returnvalue (Utilities|GetDataTableRow "/Game/Tables/TWeapons.TWeapons" _array_element)
          (:then
            (if (.ReturnValue (Utilities|Map|Find _minimal_weapon_cost (.WeaponType (Utilities|Struct|BreakWeaponStats _returnvalue))))
              (Utilities|Map|Add _minimal_weapon_cost (.WeaponType (Utilities|Struct|BreakWeaponStats _returnvalue)) (Math|Float|Min(Float) (.Value (Utilities|Map|Find _minimal_weapon_cost (.WeaponType (Utilities|Struct|BreakWeaponStats _returnvalue)))) (.Price (Utilities|Struct|BreakWeaponStats _returnvalue))))
              (else
                (Utilities|Map|Add _minimal_weapon_cost (.WeaponType (Utilities|Struct|BreakWeaponStats _returnvalue)) (.Price (Utilities|Struct|BreakWeaponStats _returnvalue)))))))))
    (:then_1
      (Utilities|Map|Clear (Variables|Private|GetMinimal%20Cabin%20Costs))
      (bind _outrownames_2 (DataTable|GetDataTableRowNames "/Game/Tables/TCabins.TCabins"))
      (for _array_element_2 _outrownames_2
        (bind _returnvalue_2 (Utilities|GetDataTableRow "/Game/Tables/TCabins.TCabins" _array_element_2)
          (:then
            (if (.ReturnValue (Utilities|Map|Find _minimal_cabin_costs (.CarName (Utilities|Struct|BreakVehiclePartStats (.PartStats (Utilities|Struct|BreakCabinFullStats _returnvalue_2))))))
              (LocalVariables|SetCache (.Value (Utilities|Map|Find _minimal_cabin_costs (.CarName (Utilities|Struct|BreakVehiclePartStats (.PartStats (Utilities|Struct|BreakCabinFullStats _returnvalue_2)))))))
              (else
                (bind _returnvalue_3 (Class|CustomFunctionLibrary|CreateObject "/Script/ExMachinaRemake.VehiclePartsCache"))
                (Utilities|Map|Add _minimal_cabin_costs (.CarName (Utilities|Struct|BreakVehiclePartStats (.PartStats (Utilities|Struct|BreakCabinFullStats _returnvalue_2)))) (.AsVehicle%20Parts%20Cache (Utilities|Casting|CastToVehiclePartsCache _returnvalue_3)))
                (LocalVariables|SetCache (.AsVehicle%20Parts%20Cache (Utilities|Casting|CastToVehiclePartsCache _returnvalue_3)))))
            (Utilities|Array|Add (Variables|/Script/ExMachinaRemake.VehiclePartsCache|GetData (LocalVariables|GetCache)) (Utilities|Struct|MakeVehiclePartsCacheData _array_element_2 (+ (.Price (Utilities|Struct|BreakVehiclePartStats (.PartStats (Utilities|Struct|BreakCabinFullStats _returnvalue_2)))) (.Value (Utilities|Map|Find (Variables|Private|GetMinimal%20Weapon%20Cost) (Utilities|Struct|BreakWeaponSlotStats (.WeaponSlots (Utilities|Struct|BreakVehiclePartStats (.PartStats (Utilities|Struct|BreakCabinFullStats _returnvalue_2))))))))))))))
    (:then_2
      (Utilities|Map|Clear (Variables|Private|GetMinimal%20Cargo%20Costs))
      (bind _outrownames_3 (DataTable|GetDataTableRowNames "/Game/Tables/TCargos.TCargos"))
      (for _array_element_3 _outrownames_3
        (bind _returnvalue_4 (Utilities|GetDataTableRow "/Game/Tables/TCargos.TCargos" _array_element_3)
          (:then
            (if (.ReturnValue (Utilities|Map|Find _minimal_cargo_costs (.CarName (Utilities|Struct|BreakVehiclePartStats (.PartStats (Utilities|Struct|BreakCargoFullStats _returnvalue_4))))))
              (LocalVariables|SetCache (.Value (Utilities|Map|Find _minimal_cargo_costs (.CarName (Utilities|Struct|BreakVehiclePartStats (.PartStats (Utilities|Struct|BreakCargoFullStats _returnvalue_4)))))))
              (else
                (bind _returnvalue_5 (Class|CustomFunctionLibrary|CreateObject "/Script/ExMachinaRemake.VehiclePartsCache"))
                (Utilities|Map|Add _minimal_cargo_costs (.CarName (Utilities|Struct|BreakVehiclePartStats (.PartStats (Utilities|Struct|BreakCargoFullStats _returnvalue_4)))) (.AsVehicle%20Parts%20Cache (Utilities|Casting|CastToVehiclePartsCache _returnvalue_5)))
                (LocalVariables|SetCache (.AsVehicle%20Parts%20Cache (Utilities|Casting|CastToVehiclePartsCache _returnvalue_5)))))
            (Utilities|Array|Add (Variables|/Script/ExMachinaRemake.VehiclePartsCache|GetData (LocalVariables|GetCache)) (Utilities|Struct|MakeVehiclePartsCacheData _array_element_3 (+ (.Price (Utilities|Struct|BreakVehiclePartStats (.PartStats (Utilities|Struct|BreakCargoFullStats _returnvalue_4)))) (.Value (Utilities|Map|Find (Variables|Private|GetMinimal%20Weapon%20Cost) (Utilities|Struct|BreakWeaponSlotStats (.WeaponSlots (Utilities|Struct|BreakVehiclePartStats (.PartStats (Utilities|Struct|BreakCargoFullStats _returnvalue_4))))))))))))))
    (:then_3
      (Utilities|Map|Clear (Variables|Private|GetMinimal%20Car%20Costs))
      (bind _outrownames_4 (DataTable|GetDataTableRowNames "/Game/Tables/TCars.TCars"))
      (for _array_element_4 _outrownames_4
        (bind _returnvalue_6 (Utilities|GetDataTableRow "/Game/Tables/TCars.TCars" _array_element_4)
          (:then
            (Utilities|Map|Add (Variables|Private|GetMinimal%20Car%20Costs) _array_element_4 (+ (Utilities|Struct|BreakF_Car_Stats _returnvalue_6) (Class|VehiclePartsCache|GetMinCost (.Value (Utilities|Map|Find (Variables|Private|GetMinimal%20Cabin%20Costs) _array_element_4))) (Class|VehiclePartsCache|GetMinCost (.Value (Utilities|Map|Find (Variables|Private|GetMinimal%20Cargo%20Costs) _array_element_4))))))))
      (Utilities|DebugOnly
        (:DebugOnly
          (Development|PrintString "Spawn Data Populated"))))))

(fn GetAliveEnemiesFactor
  (bind _outactors (Actor|GetAllActorsOfClass "/Game/Blueprints/AI/BP_AIVehiclePawn.BP_AIVehiclePawn_C"))
  (for _array_element _outactors
    (if (and (!= (Variables|/Game/Blueprints/Vehicle/BP_VehiclePawn.BP_VehiclePawn_C|GetTeam _array_element) 0) (not (Variables|/Game/Blueprints/Vehicle/BP_VehiclePawn.BP_VehiclePawn_C|GetbDead _array_element)))
      (LocalVariables|SetResult (* (LocalVariables|GetResult) (Variables|SpawnParameters|GetEnemyAliveFactor)))))
  (return (LocalVariables|GetResult)))

(fn CheckSpawnProbability
  (bind _enemyalivefactor (CallFunction|GetAliveEnemiesFactor))
  (return (Math|Random|RandomBoolwithWeight (* _enemyalivefactor (Variables|SpawnParameters|GetBaseSpawnProbability))) (Utilities|String|Append (Utilities|String|ToString(Float) (* (* _enemyalivefactor (Variables|SpawnParameters|GetBaseSpawnProbability)) 1e+02)) "%")))

(fn FindSpawnPoint
  (LocalVariables|SetCurrentMinDistance (Variables|SpawnParameters|GetMaxSpawnDistance))
  (bind _outactors (Actor|GetAllActorsOfClass "/Game/Blueprints/EnemySpawn/BP_EnemySpawnPoint.BP_EnemySpawnPoint_C"))
  (for _array_element _outactors
    (if (Math|Boolean|ANDBoolean (< (Transformation|GetDistanceTo _array_element (Game|Player|GetPlayerPawn 0)) (LocalVariables|GetCurrentMinDistance)) (> (Transformation|GetDistanceTo _array_element (Game|Player|GetPlayerPawn 0)) (Variables|SpawnParameters|GetMinSpawnDistance)) (Default|CanSpawn _array_element))
      (LocalVariables|SetCurrentMinDistance (Transformation|GetDistanceTo _array_element (Game|Player|GetPlayerPawn 0)))
      (LocalVariables|SetCurrentBestPoint _array_element)))
  (return (< (LocalVariables|GetCurrentMinDistance) (Variables|SpawnParameters|GetMaxSpawnDistance)) (LocalVariables|GetCurrentBestPoint)))

(fn CalculateEnemyPresets
  (bind _asbp_player_pawn (Utilities|Casting|CastToBP_PlayerPawn (Game|Player|GetPlayerPawn 0)))
  (LocalVariables|SetAvailable%20Cost (Default|GetCost _asbp_player_pawn))
  (LocalVariables|SetAvailable%20HP (* (.MaxHP (Utilities|Struct|BreakF_Car_Stats (Variables|/Game/Blueprints/Vehicle/BP_VehiclePawn.BP_VehiclePawn_C|GetStats _asbp_player_pawn))) 1.5))
  (Utilities|FlowControl|ForLoopwithBreak 0 (- (Variables|SpawnParameters|GetMax%20Vehicles%20Spawned) 1) :!label _label
    (:LoopBody
      (LocalVariables|SetCurrent%20Preset "")
      (Utilities|FlowControl|Sequence
        (:then_0
          ;[0.15 0.15 0.15 0.5] Car
          (bind (_car _succesfull) (CallFunction|ChoosePresetCar (LocalVariables|GetAvailable%20Cost) (LocalVariables|GetAvailable%20HP)))
          (if _succesfull
            (bind _returnvalue (Utilities|GetDataTableRow "/Game/Tables/TCars.TCars" _car)
              (:then
                (Utilities|UpdateCosts (.Price (Utilities|Struct|BreakF_Car_Stats _returnvalue))
                  (:out
                    (LocalVariables|SetAvailable%20HP (- (LocalVariables|GetAvailable%20HP) (.MaxHP (Utilities|Struct|BreakF_Car_Stats _returnvalue))))))))
            (else
              (goto _label Break))))
        (:then_1
          ;[0.15 0.15 0.15 0.5] Cabin
          (bind (_result _successfull) (CallFunction|ChoosePresetCabin (LocalVariables|GetAvailable%20Cost) _car))
          (if _successfull
            (bind _returnvalue_2 (Utilities|GetDataTableRow "/Game/Tables/TCabins.TCabins" _result)
              (:then
                (Utilities|UpdateCosts (.Price (Utilities|Struct|BreakVehiclePartStats (.PartStats (Utilities|Struct|BreakCabinFullStats _returnvalue_2)))))))
            (else
              (goto _label Break))))
        (:then_2
          ;[0.15 0.15 0.15 0.5] Cabin
          (bind (_result_2 _successfull_2) (CallFunction|ChoosePresetCargo (LocalVariables|GetAvailable%20Cost) _car))
          (if _successfull_2
            (bind _returnvalue_3 (Utilities|GetDataTableRow "/Game/Tables/TCargos.TCargos" _result_2)
              (:then
                (Utilities|UpdateCosts (.Price (Utilities|Struct|BreakVehiclePartStats (.PartStats (Utilities|Struct|BreakCargoFullStats _returnvalue_3)))))))
            (else
              (goto _label Break))))
        (:then_3
          ;[0.15 0.15 0.15 0.5] Weapons
          (bind (_result_3 _successfull_3) (CallFunction|ChoosePresetWeapon (LocalVariables|GetAvailable%20Cost) (Utilities|Struct|BreakWeaponSlotStats (.WeaponSlots (Utilities|Struct|BreakVehiclePartStats (.PartStats (Utilities|Struct|BreakCabinFullStats _returnvalue_2)))))))
          (if _successfull_3
            (bind _returnvalue_4 (Utilities|GetDataTableRow "/Game/Tables/TWeapons.TWeapons" _result_3)
              (:then
                (Utilities|UpdateCosts (Utilities|Struct|BreakWeaponStats _returnvalue_4)
                  (:out
                    _)))))
          (bind (_result_4 _successfull_4) (CallFunction|ChoosePresetWeapon (LocalVariables|GetAvailable%20Cost) (Utilities|Struct|BreakWeaponSlotStats (.WeaponSlots (Utilities|Struct|BreakVehiclePartStats (.PartStats (Utilities|Struct|BreakCargoFullStats _returnvalue_3)))))))
          (if _successfull_4
            (bind _returnvalue_5 (Utilities|GetDataTableRow "/Game/Tables/TWeapons.TWeapons" _result_4)
              (:then
                (Utilities|UpdateCosts (Utilities|Struct|BreakWeaponStats _returnvalue_5))))))
        (:then_4
          (if (CallFunction|IsPresetValid (Utilities|Struct|MakeF_VehiclePreset true _car _result _result_2 (Utilities|Array|MakeArray _result_3 _result_4)))
            (Utilities|Array|Add (LocalVariables|GetResult%20Presets) (Utilities|Struct|MakeF_VehiclePreset true _car _result _result_2 (Utilities|Array|MakeArray _result_3 _result_4)))))))
    (:Completed
      (return (LocalVariables|GetResult%20Presets) (LocalVariables|GetCost%20Used)))))

(fn ChoosePresetCar
  (params (AvailableCost :type Float%20%28double-precision%29) (AvailableHP :type Float%20%28double-precision%29))
  (bind _minimal_car_costs (Variables|Private|GetMinimal%20Car%20Costs))
  (bind _availablecars (LocalVariables|GetAvailableCars))
  (bind _keys (Utilities|Map|Keys _minimal_car_costs))
  (for _array_element _keys
    (if (<= (.Value (Utilities|Map|Find _minimal_car_costs _array_element)) AvailableCost)
      (bind _returnvalue (Utilities|GetDataTableRow "/Game/Tables/TCars.TCars" _array_element)
        (:then
          (if (<= (Utilities|Struct|BreakF_Car_Stats _returnvalue) AvailableHP)
            (Utilities|Array|Add (LocalVariables|GetAvailableCars) _array_element))))))
  (if (Utilities|Array|IsNotEmpty _availablecars)
    (return (.OutItem (Utilities|Array|Random _availablecars)) true)
    (else
      (return "None" false))))

(fn ChoosePresetCabin
  (params (AvailableCost :type Float%20%28double-precision%29) (Car :type Name))
  (bind _minimal_cabin_costs (Variables|Private|GetMinimal%20Cabin%20Costs))
  (bind _available_cabins (LocalVariables|GetAvailable%20Cabins))
  (bind (_value _returnvalue) (Utilities|Map|Find _minimal_cabin_costs Car))
  (if _returnvalue
    (for _array_element (Variables|/Script/ExMachinaRemake.VehiclePartsCache|GetData _value)
      (if (< (.minimalprice _array_element) AvailableCost)
        (Utilities|Array|Add _available_cabins (.name _array_element))))
    (if (Utilities|Array|IsNotEmpty (LocalVariables|GetAvailable%20Cabins))
      (return (.OutItem (Utilities|Array|Random _available_cabins)) true)
      (else
        _)))
  (return "None" false))

(fn ChoosePresetCargo
  (params (AvailableCost :type Float%20%28double-precision%29) (Car :type Name))
  (bind _minimal_cargo_costs (Variables|Private|GetMinimal%20Cargo%20Costs))
  (bind _availablecargos (LocalVariables|GetAvailableCargos))
  (bind (_value _returnvalue) (Utilities|Map|Find _minimal_cargo_costs Car))
  (if _returnvalue
    (for _array_element (Variables|/Script/ExMachinaRemake.VehiclePartsCache|GetData _value)
      (if (< (.minimalprice _array_element) AvailableCost)
        (Utilities|Array|Add _availablecargos (.name _array_element))))
    (if (Utilities|Array|IsNotEmpty (LocalVariables|GetAvailableCargos))
      (return (.OutItem (Utilities|Array|Random _availablecargos)) true)
      (else
        _)))
  (return "None" false))

(fn ChoosePresetWeapon
  (params (AvailableCost :type Float%20%28double-precision%29) (Type :type EWeaponType%20Enum :default "None"))
  (bind _outrownames (DataTable|GetDataTableRowNames "/Game/Tables/TWeapons.TWeapons"))
  (for _array_element _outrownames
    (bind _returnvalue (Utilities|GetDataTableRow "/Game/Tables/TWeapons.TWeapons" _array_element)
      (:then
        (if (and (Utilities|Enum|Equal(Enum) (.WeaponType (Utilities|Struct|BreakWeaponStats _returnvalue)) Type) (<= (.Price (Utilities|Struct|BreakWeaponStats _returnvalue)) AvailableCost))
          (Utilities|Array|Add (LocalVariables|GetAvailableWeapons) _array_element)))))
  (if (Utilities|Array|IsNotEmpty (LocalVariables|GetAvailableWeapons))
    (return (.OutItem (Utilities|Array|Random (LocalVariables|GetAvailableWeapons))) true)
    (else
      (return "None" false))))

(fn IsPresetValid
  (params (Preset :type F%20Vehicle%20Preset%20Structure))
  (bind (_usepreset _car _cabin _cargo _weapons) (Utilities|Struct|BreakF_VehiclePreset Preset))
  (return (Math|Boolean|ANDBoolean (!= _car "") (!= _cabin "") (!= _cargo "") (Utilities|Array|IsNotEmpty _weapons))))

(fn GetSpawnPosition
  (params (Base :type Vector) (Radius :type Float%20%28double-precision%29) (Index :type Integer) (Step :type Float%20%28double-precision%29))
  (bind _returnvalue (* Index Step))
  (return (+ Base (Math|Vector|MakeVector (* Radius (Math|Trig|Cos(Radians) _returnvalue)) (* Radius (Math|Trig|Sin(Radians) _returnvalue)) 0.0))))

(fn TrySpawnat
  (params (Location :type Vector) (Preset :type F%20Vehicle%20Preset%20Structure))
  (for _index (range 0 10)
    (bind _returnvalue (Game|SpawnActorfromClass "/Game/Blueprints/AI/BP_AIVehiclePawn.BP_AIVehiclePawn_C" (Math|Conversions|ToTransform(Vector) (+ Location (Math|Vector|MakeVector 0.0 0.0 (* (Math|Float|MakeLiteralFloat 1.5e+02) _index)))) "AdjustIfPossibleButDontSpawnIfColliding" "MultiplyWithRoot" 0 false Preset 1 "300.000000,150.000000,150.000000" 0))
    (Utilities|IsValid _returnvalue
      (:Is%20Valid
        (Default|Moveto _returnvalue (Transformation|GetActorLocation (Game|Player|GetPlayerPawn 0)))
        (return true))))
  (return false))