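; BP_SafeZone is a trigger volume that tracks whether the player pawn is inside a safe zone.
; Begin and end overlaps with BP_PlayerPawn set the PlayerInSafeZone flag on ExMachinaGameMode, printing a message in debug only.
; On BeginPlay it checks existing overlaps on its collision component, so a player who starts inside is flagged as safe.
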(event EventBeginPlay
  (CallFunction|UpdatePlayerStatus))

(event Collision|EventActorBeginOverlap
  (params (OtherActor :type Actor%20Object%20Reference))
  (Utilities|Casting|CastToBP_PlayerPawn OtherActor)
  (CallFunction|SetPlayerSafeZoneStatus true))

(event EventTick
  (params (DeltaSeconds :type Float%20%28single-precision%29)))

(event Collision|EventActorEndOverlap
  (params (OtherActor :type Actor%20Object%20Reference))
  (Utilities|Casting|CastToBP_PlayerPawn OtherActor)
  (CallFunction|SetPlayerSafeZoneStatus false))

(fn ConstructionScript)

(fn SetPlayerSafeZoneStatus
  (params (bPlayerInSafeZone :type Boolean))
  (bind _asex_machina_game_mode (Utilities|Casting|CastToExMachinaGameMode (Game|GetGameMode)))
  (bind _output_get (Variables|/Game/GameModes/ExMachinaGameMode.ExMachinaGameMode_C|SetbPlayerInSafeZone _asex_machina_game_mode bPlayerInSafeZone))
  (Utilities|DebugOnly
    (:DebugOnly
      (if _output_get
        (Development|PrintString "Player entered safe zone")
        (else
          (Development|PrintString "Player exited safe zone"))))))

(fn UpdatePlayerStatus
  (if (Utilities|Array|IsNotEmpty (Collision|GetOverlappingActors (Variables|Default|GetCollisionComponent) "/Game/Blueprints/Player/BP_PlayerPawn.BP_PlayerPawn_C" :!class /Script/Engine.PrimitiveComponent))
    (CallFunction|SetPlayerSafeZoneStatus true)))