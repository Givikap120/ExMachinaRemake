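; BP_WeaponSlot is a typed weapon slot that holds one weapon reference, along with a socket name and position loaded from slot stats.
; TrySetWeapon accepts a matching weapon type or an invalid reference, while TryDropWeapon assigns only into an empty slot.
; Assignment and removal route through SetWeapon, which signals the weapon change.
; Helper functions validate the slot setup and the held weapon's type.
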(event Custom|ReceiveBeginPlay_1)

(event Custom|ReceiveActorBeginOverlap_1
  (params (OtherActor :type Actor%20Object%20Reference)))

(event Custom|ReceiveTick_1
  (params (DeltaSeconds :type Float%20%28single-precision%29)))

(fn ConstructionScript)

(fn HasWeapon
  (return (Utilities|IsValid (Variables|Default|GetWeaponPtr))))

(fn GetWeapon
  (bind _weaponptr (Variables|Default|GetWeaponPtr))
  (Utilities|IsValid _weaponptr
    (:Is%20Valid
      (bind _asbp_weapon (Utilities|Casting|CastToBP_Weapon _weaponptr)
        (:then
          _)
        (:CastFailed
          (Development|PrintString 0 "ERROR: cast to BP Weapon failed")))
      (return _asbp_weapon))
    (:Is%20Not%20Valid
      (return 0))))

(fn TrySetWeapon
  (params (Weapon :type BP%20Weapon%20Object%20Reference))
  (Utilities|IsValid Weapon
    (:Is%20Valid
      (if (Utilities|Enum|Equal(Enum) (Variables|/Script/ExMachinaRemake.Weapon|GetWeaponType Weapon) (Variables|Default|GetSlotType))
        _
        (else
          (return false))))
    (:Is%20Not%20Valid
      _))
  (Private|SetWeapon Weapon)
  (return true))

(fn RemoveWeapon
  (if (CallFunction|HasWeapon)
    (Private|SetWeapon)
    (return true)
    (else
      (return false))))

(fn TryDropWeapon
  (params (Weapon :type BP%20Weapon%20Object%20Reference))
  (if (CallFunction|HasWeapon)
    (return false)
    (else
      (bind _succesful (CallFunction|TrySetWeapon Weapon))
      (return _succesful))))

(fn SetfromStats
  (params (Stats :type Weapon%20Slot%20Stats%20Structure))
  (Variables|Default|SetSlotType (.slottype Stats))
  (Variables|Default|SetPosX (.posx Stats))
  (Variables|Default|SetPosY (.posy Stats))
  (Variables|Default|SetSocketName (.socketname Stats)))

(fn SetWeapon
  (params (Weapon :type BP%20Weapon%20Object%20Reference))
  (Variables|Default|SetWeaponPtr Weapon)
  (Default|CallOnWeaponChanged))

(fn IsValidSlot
  (bind _socketname (Variables|Default|GetSocketName))
  (return (not (Math|Boolean|ORBoolean (== _socketname "False") (== _socketname "") (Utilities|Enum|Equal(Enum) (Variables|Default|GetSlotType) "None")))))

(fn ValidateWeapon
  (if (CallFunction|HasWeapon)
    (return (Utilities|Enum|Equal(Enum) (Variables|/Script/ExMachinaRemake.Weapon|GetWeaponType (Variables|Default|GetWeaponPtr)) (Variables|Default|GetSlotType)))
    (else
      (return true))))